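; Stage 1 player controller that applies the player's class to their player state when play begins.
; On BeginPlay, only the local controller reads PlayerClass from the PlayerState data held in BP_GameInstance and passes it to the S2C_SetClass event.
; That event casts the controller's PlayerState to BP_LostChildState and calls SetPlayerClass on it.
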(event `S2C_SetClass`
  (params (`Player Class` :type String))
  (bind _asbp_lost_child_state (cast `/Game/_Dev/Stage1/Character/Player/BP_LostChildState` (`self.PlayerState`)))
  (`/Game/_Dev/Stage1/Character/Player/BP_LostChildState.SetPlayerClass` _asbp_lost_child_state `Player Class`))

(event `self.ReceiveBeginPlay`
  (`parent.ReceiveBeginPlay`)
  (if (`self.IsLocalPlayerController`)
    (bind _asbp_game_instance (cast `/Game/_Dev/BP_GameInstance` (`GameplayStatics.GetGameInstance`)))
    (bind (_playerstate_playername _playerstate_playerclass) (break `/Game/Network/Blueprint/ST_Class` (`/Game/_Dev/BP_GameInstance.PlayerState` _asbp_game_instance)))
    (`self.S2C_SetClass` _playerstate_playerclass)))

(fn `UserConstructionScript`)