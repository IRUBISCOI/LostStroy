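; LostChild player state that stores the player's chosen class and has the player controller possess the matching Stage 1 hero.
; Shield, Sword, Bow and Wizard map to Terra, Greystone, Sparrow and Serath pawns, each found in the world with GetActorOfClass.
; SetPlayerClass stores the class name, and its OnRep possesses through the owning BP_Stage1_PlayerController.
; SetClass repeats that mapping after a short delay, using player controller 0 instead.
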(event `self.ReceiveBeginPlay`)

(event `SetClass`
  (bind _returnvalue (`GameplayStatics.GetPlayerController` 0))
  (bind _playerclass (`self.PlayerClass`))
  (`KismetSystemLibrary.Delay` 1.0)
  (`|ExecutionSequence`
    (:`then_0`
      (if (`KismetStringLibrary.EqualEqual_StrStr` _playerclass "Shield")
        (bind _returnvalue_2 (`GameplayStatics.GetActorOfClass` "/Game/_Dev/Stage1/Character/Player/LostChild_Terra.LostChild_Terra_C"))
        (`Controller.Possess` _returnvalue _returnvalue_2)))
    (:`then_1`
      (if (`KismetStringLibrary.EqualEqual_StrStr` _playerclass "Sword")
        (bind _returnvalue_3 (`GameplayStatics.GetActorOfClass` "/Game/_Dev/Stage1/Character/Player/LostChild_Greystone.LostChild_Greystone_C"))
        (`Controller.Possess` _returnvalue _returnvalue_3)))
    (:`then_2`
      (if (`KismetStringLibrary.EqualEqual_StrStr` _playerclass "Bow")
        (bind _returnvalue_4 (`GameplayStatics.GetActorOfClass` "/Game/_Dev/Stage1/Character/Player/LostChild_Sparrow.LostChild_Sparrow_C"))
        (`Controller.Possess` _returnvalue _returnvalue_4)))
    (:`then_3`
      (if (`KismetStringLibrary.EqualEqual_StrStr` _playerclass "Wizard")
        (bind _returnvalue_5 (`GameplayStatics.GetActorOfClass` "/Game/_Dev/Stage1/Character/Player/LostChild_Serath.LostChild_Serath_C"))
        (`Controller.Possess` _returnvalue _returnvalue_5)))))

(fn `OnRep_PlayerClass`
  (bind _playerclass (`self.PlayerClass`))
  (bind _asbp_stage_1_player_controller (cast `/Game/_Dev/Stage1/Character/Player/BP_Stage1_PlayerController` (`self.GetOwner`)))
  (`|ExecutionSequence`
    (:`then_0`
      (if (`KismetStringLibrary.EqualEqual_StrStr` _playerclass "Shield")
        (bind _returnvalue (`GameplayStatics.GetActorOfClass` "/Game/_Dev/Stage1/Character/Player/LostChild_Terra.LostChild_Terra_C"))
        (`Controller.Possess` _asbp_stage_1_player_controller _returnvalue)))
    (:`then_1`
      (if (`KismetStringLibrary.EqualEqual_StrStr` _playerclass "Sword")
        (bind _returnvalue_2 (`GameplayStatics.GetActorOfClass` "/Game/_Dev/Stage1/Character/Player/LostChild_Greystone.LostChild_Greystone_C"))
        (`Controller.Possess` _asbp_stage_1_player_controller _returnvalue_2)))
    (:`then_2`
      (if (`KismetStringLibrary.EqualEqual_StrStr` _playerclass "Bow")
        (bind _returnvalue_3 (`GameplayStatics.GetActorOfClass` "/Game/_Dev/Stage1/Character/Player/LostChild_Sparrow.LostChild_Sparrow_C"))
        (`Controller.Possess` _asbp_stage_1_player_controller _returnvalue_3)))
    (:`then_3`
      (if (`KismetStringLibrary.EqualEqual_StrStr` _playerclass "Wizard")
        (bind _returnvalue_4 (`GameplayStatics.GetActorOfClass` "/Game/_Dev/Stage1/Character/Player/LostChild_Serath.LostChild_Serath_C"))
        (`Controller.Possess` _asbp_stage_1_player_controller _returnvalue_4)))))

(fn `SetPlayerClass`
  (params (PlayerClass :type String))
  (set `self.PlayerClass` PlayerClass))

(fn `UserConstructionScript`)