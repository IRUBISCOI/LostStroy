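; Enemy spawner actor that periodically spawns batches of BP_Zombie during a stage.
; BeginPlay starts a timer for SpawnZombie, which places each zombie with random yaw at a random reachable navmesh point within its Sphere radius.
; SpawnZombie re-arms the timer only while the running total is under a cap, checked per batch, so spawning then stops.
; The StageClear event destroys the spawner.
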(event `self.ReceiveBeginPlay`
  (`KismetSystemLibrary.K2_SetTimer` null "SpawnZombie" 5.0))

(event `/Game/_Dev/Stage1/Blueprints/KillInterface.StageClear`
  (`self.K2_DestroyActor`))

(fn `SpawnZombie`
  (if (< (`self.ZombieCount`) 10)
    (for _ (range 4)
      (`/Engine/EditorBlueprintResources/StandardMacros.IncrementInt` (`self.ZombieCount`)
        (:`  `
          (`|SpawnActorFromClass` "/Game/_Dev/Stage1/Character/Enemy/BP_Zombie.BP_Zombie_C" (`KismetMathLibrary.MakeTransform` (`NavigationSystemV1.K2_GetRandomReachablePointInRadius` (`self.K2_GetActorLocation`) (`SphereComponent.SphereRadius` (`self.Sphere`)) null null) (`KismetMathLibrary.MakeRotator` 0.0 0.0 (`KismetMathLibrary.RandomFloatInRange` 0.0 360.0))) "AlwaysSpawn" "OverrideRootScale" null null))))
    (`KismetSystemLibrary.K2_SetTimer` null "SpawnZombie" 5.0)))

(fn `UserConstructionScript`)