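; Stage 1 game state that tracks the kill goal and triggers the boss encounter once it is met.
; The TotalKill RepNotify updates kill messages through KillInterface and the HUD, then broadcasts stage clear when the target is reached.
; After a short timer, the authority spawns the boss at a TargetPoint and stops its AI logic.
; A second timer then plays the intro cinematic and switches the first player controller's view to it.
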(event `Res_BossZoomIn`
  ;[1 1 1] 시퀸스 실행
  (bind _outactor (`LevelSequencePlayer.CreateLevelSequencePlayer` "/Game/_Dev/Stage1/Blueprints/HJH_CineIntroSeqRev.HJH_CineIntroSeqRev"))
  (`MovieSceneSequencePlayer.PlayTo` :`self` (`LevelSequenceActor.SequencePlayer` _outactor))
  (`PlayerController.SetViewTargetWithBlend` (`GameplayStatics.GetPlayerController` 0) _outactor 0.0 "VTBlend_Linear" 0.0 false))

(fn `OnRep_TotalKill`
  (`|ExecutionSequence`
    (:`then_0`
      (bind _outactors (`GameplayStatics.GetAllActorsWithInterface` "/Game/_Dev/Stage1/Blueprints/KillInterface.KillInterface_C"))
      (`|ExecutionSequence`
        (:`then_0`
          (message `/Game/_Dev/Stage1/Blueprints/KillInterface.UpdateKill` _outactors))
        (:`then_1`
          (bind _asgame_hud (cast `GameHUD` (`PlayerController.GetHUD` (`GameplayStatics.GetPlayerController` 0))))
          (message `/Game/_Dev/Stage1/Blueprints/KillInterface.UpdateKill` _asgame_hud))))
    (:`then_1`
      (if (>= (`self.TotalKill`) (`self.CompleteKill`))
        (`self.Stage 1 Complete`)))))

(fn `SpawnBoss`
  (`/Engine/EditorBlueprintResources/ActorMacros.Switch Has Authority`
    (:`Authority`
      (bind _returnvalue (`GameplayStatics.GetActorOfClass` "/Script/Engine.TargetPoint"))
      ;[1 1 1] 보스 소환
      (bind _returnvalue_2 (`|SpawnActorFromClass` "/Game/_Dev/Stage1/Character/Enemy/BP_SpawnBoss.BP_SpawnBoss_C" (`KismetMathLibrary.MakeTransform` (`self.K2_GetActorLocation` _returnvalue) (struct :`Yaw` 90.0) (2.0 2.0 2.0)) "Undefined" "OverrideRootScale" null null))
      (bind _returnvalue_3 (`AIBlueprintHelperLibrary.GetAIController` _returnvalue_2))
      ;[1 1 1] 보스 잠시 멈춤
      (`/Engine/EditorBlueprintResources/StandardMacros.IsValid` _returnvalue_3
        (:`Is Valid`
          (`BrainComponent.StopLogic` (`AIController.BrainComponent` _returnvalue_3) "Spawn")
          ;[1 1 1] 시퀸서 길이만큼만 실행
          (`KismetSystemLibrary.K2_SetTimer` null "ZoomInBoss" 2.38))))))

(fn `Stage 1 Complete`
  (`|ExecutionSequence`
    (:`then_0`
      (bind _outactors (`GameplayStatics.GetAllActorsWithInterface` "/Game/_Dev/Stage1/Blueprints/KillInterface.KillInterface_C"))
      (for _array_element _outactors
        (message `/Game/_Dev/Stage1/Blueprints/KillInterface.StageClear` _array_element)))
    (:`then_1`
      (bind _aslost_child_player_base (cast `/Game/_Dev/Stage1/Character/Player/LostChildPlayerBase` (`GameplayStatics.GetPlayerCharacter` 0)))
      (`/Game/_Dev/Stage1/Character/Player/LostChildPlayerBase.ClearStage` _aslost_child_player_base))
    (:`then_2`
      (`KismetSystemLibrary.K2_SetTimer` null "SpawnBoss" 2.0))))

(fn `UserConstructionScript`)

(fn `ZoomInBoss`
  (`self.Res_BossZoomIn`))