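; BP_Weapon is a weapon actor that plays the owning LostChild player's shoot and reload animations in response to trigger and reload input events.
; PressTrigger casts OwnChar to LostChildPlayer and plays its ShootMontage when pressed, ignoring release.
; PressReload first checks that the owner is valid and its LostChildState reports a usable magazine, then plays the ReloadMontage.
; The graph itself only drives montages, with no firing or ammo-change logic.
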(event `WeaponInterface.PressTrigger`
  (params (isPressed :type Boolean))
  (if isPressed
    (bind _aslost_child_player (cast `LostChildPlayer` (`self.OwnChar`)))
    (`Character.PlayAnimMontage` _aslost_child_player (`LostChildPlayer.ShootMontage` _aslost_child_player) 1.0 "None")))

(event `WeaponInterface.PressReload`
  (bind _ownchar (`self.OwnChar`))
  (`/Engine/EditorBlueprintResources/StandardMacros.IsValid` _ownchar
    (:`Is Valid`
      (bind _aslost_child_state (cast `LostChildState` (`Pawn.PlayerState` _ownchar)))
      (if (`LostChildState.IsCanUseMag` _aslost_child_state)
        (bind _aslost_child_player (cast `LostChildPlayer` _ownchar))
        (`Character.PlayAnimMontage` _aslost_child_player (`LostChildPlayer.ReloadMontage` _aslost_child_player) 1.0 "None")))))

(fn `UserConstructionScript`)