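; Burst weapon Blueprint that repeats the owning LostChildPlayer's shoot montage while the trigger is held.
; Pressing the trigger plays the montage at once and starts a looping named timer on NotifyShootMontage, which is cleared on release, on detach, or when BurstShooting finds no valid owner.
; Reload plays the character's reload montage only if the LostChildState player state reports a usable magazine.
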(event `self.BurstShooting`
  (`/Engine/EditorBlueprintResources/StandardMacros.IsValid` (`self.GetOwner`)
    (:`Is Not Valid`
      (`KismetSystemLibrary.K2_ClearTimer` null "NotifyShootMontage" :!label _label))))

(event `WeaponInterface.PressTrigger`
  (params (isPressed :type Boolean))
  (if isPressed
    (`|ExecutionSequence`
      (:`then_0`
        (`self.NotifyShootMontage`))
      (:`then_1`
        (`KismetSystemLibrary.K2_SetTimer` null "NotifyShootMontage" 0.2 true)))
    (else
      (goto _label))))

(event `WeaponInterface.DetachWeapon`
  (params (targetChar :type "Character Object Reference"))
  (`parent.DetachWeapon` targetChar)
  (goto _label))

(event `WeaponInterface.PressReload`
  (bind _ownchar (`self.OwnChar`))
  (`/Engine/EditorBlueprintResources/StandardMacros.IsValid` _ownchar
    (:`Is Valid`
      (bind _aslost_child_state (cast `LostChildState` (`Pawn.PlayerState` _ownchar)))
      (if (`LostChildState.IsCanUseMag` _aslost_child_state)
        (bind _aslost_child_player (cast `LostChildPlayer` _ownchar))
        (`Character.PlayAnimMontage` _aslost_child_player (`LostChildPlayer.ReloadMontage` _aslost_child_player) 1.0 "None")))))

(fn `NotifyShootMontage`
  (bind _aslost_child_player (cast `LostChildPlayer` (`self.OwnChar`)))
  (`Character.PlayAnimMontage` _aslost_child_player (`LostChildPlayer.ShootMontage` _aslost_child_player) 1.0 "None"))

(fn `UserConstructionScript`)