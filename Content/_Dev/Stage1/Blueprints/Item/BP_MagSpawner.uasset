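; BP_MagSpawner is a Stage 1 item spawner that periodically drops batches of BP_MagObject pickups around itself.
; A timer started on BeginPlay calls SpawnMag, which re-arms the same timer after each batch.
; Each object spawns at a random reachable navigation point within the Sphere radius, raised slightly with random yaw and ignoring collisions.
; The StageClear event destroys the spawner.
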(event `self.ReceiveBeginPlay`
  (`KismetSystemLibrary.K2_SetTimer` null "SpawnMag" 5.0))

(event `/Game/_Dev/Stage1/Blueprints/KillInterface.StageClear`
  (`self.K2_DestroyActor`))

(fn `SpawnMag`
  (for _ (range 4)
    (`|SpawnActorFromClass` "/Game/_Dev/Stage1/Blueprints/Item/BP_MagObject.BP_MagObject_C" (`KismetMathLibrary.MakeTransform` (+ (`NavigationSystemV1.K2_GetRandomReachablePointInRadius` (`self.K2_GetActorLocation`) (`SphereComponent.SphereRadius` (`self.Sphere`)) null null) (0.0 0.0 75.0)) (`KismetMathLibrary.MakeRotator` 0.0 0.0 (`KismetMathLibrary.RandomFloatInRange` 0.0 360.0))) "AlwaysSpawn" "OverrideRootScale" null null))
  (`KismetSystemLibrary.K2_SetTimer` null "SpawnMag" 5.0))

(fn `UserConstructionScript`)