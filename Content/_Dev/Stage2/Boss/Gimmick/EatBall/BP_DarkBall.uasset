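; Dark ball hazard for the Stage 2 boss's EatBall gimmick that poisons a player on contact.
; Overlapping a BP_Player_Base applies poison-type damage with a timed damage debuff, plays an explosion sound and destroys the ball.
; The Destroyed event spawns a scaled-down thunder-ball hit effect, so it accompanies any removal.
; Older damage variants remain as disconnected nodes, and the PoisonEffect graph is not called here.
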(event `self.ReceiveActorBeginOverlap`
  (params (OtherActor :type "Actor Object Reference"))
  (bind _asbp_player_base (cast `/Game/_Dev/Stage2/Char/BP_Player_Base` OtherActor))
  (`self.TakeDamage` _asbp_player_base 50.0 "/Game/BossAIToolkit/Blueprints/DamageTypes/BP_DamageType_Poison.BP_DamageType_Poison_C" "NewEnumerator2" 10.0 5.0)
  (`GameplayStatics.PlaySoundAtLocation` "/Game/StarterContent/Audio/Explosion01.Explosion01" (`self.K2_GetActorLocation` _asbp_player_base) (struct) 1.0 1.0 0.0 null null null)
  (`self.K2_DestroyActor`))

(event `self.ReceiveDestroyed`
  (`GameplayStatics.SpawnEmitterAtLocation` "/Game/FXVarietyPack/Particles/P_ky_ThunderBallHit.P_ky_ThunderBallHit" (`self.K2_GetActorLocation`) (`self.K2_GetActorRotation`) (0.5 0.5 0.5)))

(fn `PoisonEffect`
  (params (InputPin :type "Actor Object Reference"))
  (bind _asbp_player_base (cast `/Game/_Dev/Stage2/Char/BP_Player_Base` InputPin))
  (`GameplayStatics.ApplyPointDamage` _asbp_player_base 100.0 (`self.K2_GetActorLocation` InputPin) (`GameplayStatics.MakeHitResult` false) null null "/Game/BossAIToolkit/Blueprints/DamageTypes/BP_DamageType_Poison.BP_DamageType_Poison_C"))

(fn `UserConstructionScript`)