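; Boss "EatBall" gimmick spawner that emits random balls in random directions on a looping timer until shortly before its lifespan ends.
; Balls become visible on leaving VisibleSphere, and item objects are destroyed on leaving DestroySphere.
; A delay after spawning begins advances the boss phase.
; On destruction it scatters explosions, and the server deals max-health damage to players inside DestroySphere, unless CriticalShield is at least two, which is consumed instead.
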(event `self.ReceiveBeginPlay`
  (`self.Req_SpawnBallStart`))

(event `Req_SpawnBallStart`
  (`self.SetLifeSpan` (`self.In Lifespan`))
  (`KismetSystemLibrary.K2_SetTimer` null "SpawnBall" 0.2 true)
  (`KismetSystemLibrary.K2_SetTimerDelegate` (delegate `ClearTimer`) (- (`self.In Lifespan`) 1.0)))

(event `ClearTimer`
  (`KismetSystemLibrary.K2_ClearTimer` null "SpawnBall"))

(event `self.DestroySphere.OnComponentEndOverlap`
  (params (OverlappedComponent :type "PrimitiveComponent Object Reference") (OtherActor :type "Actor Object Reference") (OtherComp :type "PrimitiveComponent Object Reference") (OtherBodyIndex :type Integer))
  (bind _asitem_object (cast `ItemObject` OtherActor))
  (`self.K2_DestroyActor` _asitem_object))

(event `self.VisibleSphere.OnComponentEndOverlap`
  (params (OverlappedComponent :type "PrimitiveComponent Object Reference") (OtherActor :type "Actor Object Reference") (OtherComp :type "PrimitiveComponent Object Reference") (OtherBodyIndex :type Integer))
  (bind _asbp_ball_base (cast `/Game/_Dev/Stage2/Boss/Gimmick/EatBall/BP_BallBase` OtherActor))
  (`SceneComponent.SetVisibility` (`ItemObject.StaticMesh` _asbp_ball_base) true false)
  (`ActorComponent.SetActive` (`/Game/_Dev/Stage2/Boss/Gimmick/EatBall/BP_BallBase.Particle` _asbp_ball_base) true false))

(event `SpawnBall`
  (bind _returnvalue (`self.K2_GetActorLocation`))
  (`|SpawnActorFromClass` (`KismetArrayLibrary.Array_Random` (`self.BallList`)) (`KismetMathLibrary.MakeTransform` _returnvalue (`KismetMathLibrary.MakeRotator` 0.0 0.0 (`KismetMathLibrary.RandomFloatInRange` 0.0 360.0))) "Undefined" "OverrideRootScale" null null)
  (`GameplayStatics.PlaySoundAtLocation` "/Game/_Dev/Stage2/Boss/Blueprint/Sound/SpawnSoundQue.SpawnSoundQue" _returnvalue (struct) 0.5 1.0 0.0 null null null)
  (if (not (`self.IsTriggered`))
    ;[1 1 1] 보스 다음 단계로
    (`KismetSystemLibrary.Delay` (- (`self.In Lifespan`) 1.0))
    (bind _outactors (`GameplayStatics.GetAllActorsOfClass` "/Game/_Dev/Stage2/Boss/Blueprint/NewBoss.NewBoss_C"))
    (`/Game/BossAIToolkit/Blueprints/BPC_Boss_Behavior.TriggerNextPhase` (`/Game/BossAIToolkit/Blueprints/BP_Boss_Base.Boss Behavior` (`|GetArrayItem` _outactors)))
    (set `self.IsTriggered` true)))

(event `self.ReceiveDestroyed`
  (bind _destroysphere (`self.DestroySphere`))
  (`|ExecutionSequence`
    (:`then_0`
      (for _ (range 50)
        (`GameplayStatics.SpawnEmitterAtLocation` "/Game/BossAIToolkit/Demo/FX/Particles/P_Explosion.P_Explosion" (`NavigationSystemV1.K2_GetRandomReachablePointInRadius` (`self.K2_GetActorLocation`) (`SphereComponent.SphereRadius` (`self.DestroySphere`)) null null) (`KismetMathLibrary.MakeRotator` 0.0 0.0 (`KismetMathLibrary.RandomFloatInRange` 0.0 360.0)))))
    (:`then_1`
      (`/Engine/EditorBlueprintResources/ActorMacros.Switch Has Authority`
        (:`Authority`
          (for _array_element (`PrimitiveComponent.GetOverlappingActors` _destroysphere null)
            (bind _asbp_player_base (cast `/Game/_Dev/Stage2/Char/BP_Player_Base` _array_element))
            ;[1 1 1] 즉사
            (`ActorComponent.SetActive` (`/Game/_Dev/Stage2/Char/BP_Player_Base.ParticleSystem_Buff1` _asbp_player_base) false false)
            (`ActorComponent.SetActive` (`/Game/_Dev/Stage2/Char/BP_Player_Base.ParticleSystem_Buff2` _asbp_player_base) false false)
            ;;[1 1 1] 즉사 조건 미기입
            (if (< (`/Game/_Dev/Stage2/Char/BP_Player_Base.CriticalShield` _asbp_player_base) 2)
              (`/Game/_Dev/Stage2/Char/BP_Player_Base.TakeDamage` _asbp_player_base (`/Game/_Dev/Stage2/Char/BP_Player_Base.MaxHealth` _asbp_player_base) null (`SceneComponent.K2_GetComponentLocation` _destroysphere) false)
              (else
                (set `/Game/_Dev/Stage2/Char/BP_Player_Base.CriticalShield` 0 _asbp_player_base)))))))))

(fn `UserConstructionScript`)