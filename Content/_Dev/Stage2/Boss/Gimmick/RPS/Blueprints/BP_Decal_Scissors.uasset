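; Short-lived scissors zone for the Stage 2 boss rock-paper-scissors gimmick, removing itself after about five seconds.
; Its sphere affects only players whose RandomRPS value is 2.
; A component hit turns on the player's CriticalShield and second buff particle system.
; A begin overlap turns both off, so the shield state depends on which collision event fires.
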(event `self.ReceiveBeginPlay`
  (`self.SetLifeSpan` 5.1))

(event `self.Sphere.OnComponentHit`
  (params (HitComponent :type "PrimitiveComponent Object Reference") (OtherActor :type "Actor Object Reference") (OtherComp :type "PrimitiveComponent Object Reference") (NormalImpulse :type "Vector Structure") (Hit :type "HitResult Structure (by ref)"))
  (bind _asbp_player_base (cast `/Game/_Dev/Stage2/Char/BP_Player_Base` OtherActor))
  (if (== (`/Game/_Dev/Stage2/Char/BP_Player_Base.RandomRPS` _asbp_player_base) 2)
    (set `/Game/_Dev/Stage2/Char/BP_Player_Base.CriticalShield` 1 _asbp_player_base)
    (`ActorComponent.SetActive` (`/Game/_Dev/Stage2/Char/BP_Player_Base.ParticleSystem_Buff2` _asbp_player_base) true false)))

(event `self.Sphere.OnComponentBeginOverlap`
  (params (OverlappedComponent :type "PrimitiveComponent Object Reference") (OtherActor :type "Actor Object Reference") (OtherComp :type "PrimitiveComponent Object Reference") (OtherBodyIndex :type Integer) (bFromSweep :type Boolean) (SweepResult :type "HitResult Structure (by ref)"))
  (bind _asbp_player_base (cast `/Game/_Dev/Stage2/Char/BP_Player_Base` OtherActor))
  (if (== (`/Game/_Dev/Stage2/Char/BP_Player_Base.RandomRPS` _asbp_player_base) 2)
    (set `/Game/_Dev/Stage2/Char/BP_Player_Base.CriticalShield` 0 _asbp_player_base)
    (`ActorComponent.SetActive` (`/Game/_Dev/Stage2/Char/BP_Player_Base.ParticleSystem_Buff2` _asbp_player_base) false false)))

(fn `UserConstructionScript`)