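; Player state for Stage 2 that stores the player's chosen class and gives the controller the matching top-down character.
; SetPlayerClass writes PlayerClass; its OnRep casts the owner to BP_TopDownController, printing a debug owner name first.
; The OnRep possesses the first placed Shield, Sword, Bow or Magic character found for that class, then calls INITUI on player character 0.
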(fn `OnRep_PlayerClass`
  (bind _returnvalue (`self.GetOwner`))
  (bind _playerclass (`self.PlayerClass`))
  (`KismetSystemLibrary.PrintString` (`KismetStringLibrary.Concat_StrStr` "owner : " (`KismetSystemLibrary.GetDisplayName` _returnvalue)) true true (struct :`R` 1.0 :`G` 0.03643 :`A` 1.0) 60.0)
  (bind _asbp_top_down_controller (cast `/Game/_Dev/Stage2/Char/BP_TopDownController` _returnvalue))
  (`|ExecutionSequence`
    (:`then_0`
      (if (`KismetStringLibrary.EqualEqual_StrStr` _playerclass "Shield")
        (bind _returnvalue_2 (`GameplayStatics.GetActorOfClass` "/Game/_Dev/Stage2/Char/Shield/BP_TopDownCharacter_Shield.BP_TopDownCharacter_Shield_C"))
        (`Controller.Possess` _asbp_top_down_controller _returnvalue_2)
        (bind _asbp_player_base (cast `/Game/_Dev/Stage2/Char/BP_Player_Base` (`GameplayStatics.GetPlayerCharacter` 0) :!label _label))
        (`/Game/_Dev/Stage2/Char/BP_Player_Base.INITUI` _asbp_player_base)))
    (:`then_1`
      (if (`KismetStringLibrary.EqualEqual_StrStr` _playerclass "Sword")
        (bind _returnvalue_3 (`GameplayStatics.GetActorOfClass` "/Game/_Dev/Stage2/Char/Sword/BP_TopDownCharacter_Sword.BP_TopDownCharacter_Sword_C"))
        (`Controller.Possess` _asbp_top_down_controller _returnvalue_3)
        (goto _label)))
    (:`then_2`
      (if (`KismetStringLibrary.EqualEqual_StrStr` _playerclass "Bow")
        (bind _returnvalue_4 (`GameplayStatics.GetActorOfClass` "/Game/_Dev/Stage2/Char/Bow/BP_TopDownCharacter_Bow.BP_TopDownCharacter_Bow_C"))
        (`Controller.Possess` _asbp_top_down_controller _returnvalue_4)
        (goto _label)))
    (:`then_3`
      (if (`KismetStringLibrary.EqualEqual_StrStr` _playerclass "Wizard")
        (bind _returnvalue_5 (`GameplayStatics.GetActorOfClass` "/Game/_Dev/Stage2/Char/Magic/BP_TopDownCharacter_Magic.BP_TopDownCharacter_Magic_C"))
        (`Controller.Possess` _asbp_top_down_controller _returnvalue_5)
        (goto _label)))))

(fn `SetPlayerClass`
  (params (PlayerClass :type String))
  (set `self.PlayerClass` PlayerClass))

(fn `UserConstructionScript`)