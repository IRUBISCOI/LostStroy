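; Player HUD Blueprint that shows a randomly picked rock-paper-scissors symbol when play begins.
; On BeginPlay it creates a BP_RPS_HUD widget, collapses the two symbols that do not match the roll and adds the widget to the viewport.
; RandomInteger(2) only yields 0 or 1, so Rock or Paper appears and the Scissors branch is never taken.
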(event `self.ReceiveBeginPlay`
  (bind _output_get (set `self.Random_RPS` (`KismetMathLibrary.RandomInteger` 2)))
  (bind _returnvalue (`|CreateWidget` "/Game/_Dev/Stage2/Boss/Gimmick/RPS/Blueprints/BP_RPS_HUD.BP_RPS_HUD_C"))
  (bind _output_get_2 (set `self.RPS` _returnvalue))
  (`|ExecutionSequence`
    (:`then_0`
      (if (== _output_get 0)
        (`Widget.SetVisibility` (`/Game/_Dev/Stage2/Boss/Gimmick/RPS/Blueprints/BP_RPS_HUD.Scissors` _output_get_2) "Collapsed")
        (`Widget.SetVisibility` (`/Game/_Dev/Stage2/Boss/Gimmick/RPS/Blueprints/BP_RPS_HUD.Paper` _output_get_2) "Collapsed")
        (`UserWidget.AddToViewport` (`self.RPS`) 0 :!label _label)))
    (:`then_1`
      (if (== _output_get 1)
        (bind _rock (`/Game/_Dev/Stage2/Boss/Gimmick/RPS/Blueprints/BP_RPS_HUD.Rock` _output_get_2))
        (`Widget.SetVisibility` _rock "Collapsed")
        (`Widget.SetVisibility` (`/Game/_Dev/Stage2/Boss/Gimmick/RPS/Blueprints/BP_RPS_HUD.Scissors` _output_get_2) "Collapsed")
        (goto _label)))
    (:`then_2`
      (if (== _output_get 2)
        (`Widget.SetVisibility` _rock "Collapsed")
        (`Widget.SetVisibility` (`/Game/_Dev/Stage2/Boss/Gimmick/RPS/Blueprints/BP_RPS_HUD.Paper` _output_get_2) "Collapsed")
        (goto _label)))))