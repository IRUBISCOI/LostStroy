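; BP_PC is a player controller for Stage 2 with a visible mouse cursor, click-to-move and a default attack.
; While the move input is held, Tick traces under the cursor and runs SimpleMoveToLocation to that point.
; Clients send the goal to the server and also move locally, with debug prints on each path.
; Attack input calls AttackBase on the cached BP_Player_Base, re-fetching it if invalid.
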(event `self.ReceiveBeginPlay`
  (set `self.bShowMouseCursor` true)
  (bind _asbp_player_base (cast `/Game/_Dev/Stage2/Char/BP_Player_Base` (`GameplayStatics.GetPlayerCharacter` 0)))
  (set `self.BP_Player_Base` _asbp_player_base))

(event `Server_Move`
  (params (Controller :type "Controller Object Reference") (Goal :type "Vector Structure (by ref)"))
  (`AIBlueprintHelperLibrary.SimpleMoveToLocation` Controller Goal))

(event `self.ReceiveTick`
  (params (DeltaSeconds :type "Float (single-precision)"))
  (if (`self.NewVar_0`)
    (`/Engine/EditorBlueprintResources/ActorMacros.Switch Has Authority`
      (:`Authority`
        (`KismetSystemLibrary.PrintString` "server")
        (`AIBlueprintHelperLibrary.SimpleMoveToLocation` self (`.Location` (`GameplayStatics.BreakHitResult` (`self.GetHitResultUnderCursorByChannel` "TraceTypeQuery1")))))
      (:`Remote`
        (`KismetSystemLibrary.PrintString` "client")
        (`self.Server_Move` self (`.Location` (`GameplayStatics.BreakHitResult` (`self.GetHitResultUnderCursorByChannel` "TraceTypeQuery1"))))
        (`AIBlueprintHelperLibrary.SimpleMoveToLocation` self (`.Location` (`GameplayStatics.BreakHitResult` (`self.GetHitResultUnderCursorByChannel` "TraceTypeQuery1"))))))
    (else
      (`KismetSystemLibrary.PrintString` "Hello"))))

(event `InputAction|Stage2_CharacterMove` :consume false :overrideparent false
  (params (Key :type "Key Structure"))
  (:`Pressed`
    (set `self.NewVar_0` true))
  (:`Released`
    (set `self.NewVar_0` false)))

(event `InputAction|Stage2_DefaultAttack`
  (params (Key :type "Key Structure"))
  (:`Pressed`
    (`/Engine/EditorBlueprintResources/StandardMacros.IsValid` (`self.BP_Player_Base`)
      (:`Is Valid`
        _)
      (:`Is Not Valid`
        (bind _asbp_player_base (cast `/Game/_Dev/Stage2/Char/BP_Player_Base` (`GameplayStatics.GetPlayerCharacter` 0)))
        (set `self.BP_Player_Base` _asbp_player_base)))
    (`/Game/_Dev/Stage2/Char/BP_Player_Base.Attack_Base` (`self.BP_Player_Base`))))

(fn `UserConstructionScript`)