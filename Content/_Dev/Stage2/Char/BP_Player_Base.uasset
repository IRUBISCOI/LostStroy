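; Base player character for a networked boss-fight game, with mouse-aimed combo attacks, dash, dodge roll, blocking and boss lock-on.
; Combat actions route through Server events, with montage notifies gating damage and combo steps while stamina is spent and timer-regenerated.
; Incoming damage passes through damage-type processing and directional block checks into hit reacts or ragdoll death.
; It also creates player and boss health UI and applies crowd control and debuffs via a status-effect component.
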(event `BossUI_Remove`
  (`Widget.RemoveFromParent` (`self.BossUI`)))

(event `PlayerUI_Remove`
  (`Widget.RemoveFromParent` (`self.PlayerUIRef`)))

(event `INITUI`
  ;[1 1 1] Initialize references
  (bind _returnvalue (`GameplayStatics.GetActorOfClass` "/Game/BossAIToolkit/Blueprints/BP_BossAIStorage.BP_BossAIStorage_C" :!label _label))
  (message `/Game/BossAIToolkit/Blueprints/Interfaces/BI_AIStorage.BossAddActorToList` _returnvalue self)
  (set `self.TargetRotation` (`self.K2_GetActorRotation`))
  (set `self.Health` (`self.MaxHealth`))
  (set `self.Stamina` (`self.MaxStamina`))
  (bind _asplayer_controller (cast `PlayerController` (`self.GetController`)))
  (bind _output_get (set `self.ControllerRef` _asplayer_controller))
  ;[1 1 1] Create Player HUD and UI
  (bind _returnvalue_2 (`|CreateWidget` "/Game/_Dev/Stage2/Char/Widgets/WB_PlayerUI2.WB_PlayerUI2_C" _output_get))
  (bind _output_get_2 (set `self.PlayerUIRef` _returnvalue_2))
  (`UserWidget.AddToViewport` _output_get_2 0)
  (bind _outactors (`GameplayStatics.GetAllActorsOfClass` "/Game/BossAIToolkit/Blueprints/BP_Boss_Base.BP_Boss_Base_C"))
  (`PanelWidget.ClearChildren` (`/Game/_Dev/Stage2/Char/Widgets/WB_PlayerUI2.BossBarBox` (`self.PlayerUIRef`)))
  (for _array_element _outactors
    (bind _returnvalue_3 (`|CreateWidget` "/Game/BossAIToolkit/Blueprints/Widgets/WB_BossHealth.WB_BossHealth_C" (`self.ControllerRef`)))
    (set `self.BossUI` _returnvalue_3)
    (set `/Game/BossAIToolkit/Blueprints/Widgets/WB_BossHealth.BossBehaviorRef` (`/Game/BossAIToolkit/Blueprints/BP_Boss_Base.Boss Behavior` _array_element) _returnvalue_3)
    (`VerticalBox.AddChildToVerticalBox` (`/Game/_Dev/Stage2/Char/Widgets/WB_PlayerUI2.BossBarBox` (`self.PlayerUIRef`)) _returnvalue_3)))

(event `self.ReceiveBeginPlay`
  ;[1 1 1] Initialize references
  (`|ExecutionSequence`
    (:`then_0`
      (goto _label))
    (:`then_1`
      (`KismetSystemLibrary.Delay` 0.2)
      (bind _asydygame_state (cast `/Game/Network/Blueprint/YDYGameState` (`GameplayStatics.GetGameState`)))
      (set `self.RandomRPS` (`/Game/Network/Blueprint/YDYGameState.Rand_RPS` _asydygame_state)))))

(event `Attack_Base`
  (`self.Attack Auto Mouse Lock On`)
  ;[1 0 0] Light and heavt attack inputs
  (if (not (`self.IsAttacking`))
    (`self.Server_OnAttack` "NewEnumerator1")))

(event `self.ReceivePointDamage`
  (params (Damage :type "Float (single-precision)") (DamageType :type "DamageType Object Reference") (HitLocation :type "Vector Structure") (HitNormal :type "Vector Structure") (HitComponent :type "PrimitiveComponent Object Reference") (BoneName :type Name) (ShotFromDirection :type "Vector Structure") (InstigatedBy :type "Controller Object Reference") (DamageCauser :type "Actor Object Reference") (HitInfo :type "HitResult Structure (by ref)"))
  (bind _blocked (`self.CheckBlock` ShotFromDirection))
  ;[1 1 1] Player take damage
  (bind _newdamage (message `/Game/BossAIToolkit/Blueprints/Interfaces/BI_DamageType.ProcessDamage` DamageType self Damage _blocked DamageCauser))
  (`self.TakeDamage` _newdamage DamageType ShotFromDirection _blocked))

(event `self.ReceiveRadialDamage`
  (params (DamageReceived :type "Float (single-precision)") (DamageType :type "DamageType Object Reference") (Origin :type "Vector Structure") (HitInfo :type "HitResult Structure (by ref)") (InstigatedBy :type "Controller Object Reference") (DamageCauser :type "Actor Object Reference"))
  (bind _blocked (`self.CheckBlock` Origin))
  ;[1 1 1] Player take damage
  (bind _newdamage (message `/Game/BossAIToolkit/Blueprints/Interfaces/BI_DamageType.ProcessDamage` DamageType self DamageReceived _blocked DamageCauser))
  (`self.TakeDamage` _newdamage DamageType Origin _blocked))

(event `InputAction|Stage2_SkillA`
  (params (Key :type "Key Structure"))
  ;[1 1 1] 코멘트
)

(event `OnDeath`
  (bind _playeruiref (`self.PlayerUIRef`))
  (bind _bossui (`self.BossUI`))
  (bind _mesh (`self.Mesh`))
  ;[1 1 1] On player death, activate ragdoll
  (set `self.IsDead` true)
  (set `self.IsAttacking` false)
  (`KismetArrayLibrary.Array_Clear` (`self.Tags`))
  (`PrimitiveComponent.SetSimulatePhysics` _mesh true)
  (`PrimitiveComponent.SetCollisionProfileName` _mesh "Ragdoll" true)
  (`/Engine/EditorBlueprintResources/StandardMacros.IsValid` _playeruiref
    (:`Is Valid`
      (`Widget.RemoveFromParent` _playeruiref)
      (`/Engine/EditorBlueprintResources/StandardMacros.IsValid` _bossui
        (:`Is Valid`
          (`Widget.RemoveFromParent` _bossui))))))

(event `Hit_Anim_Blocking`)

(event `Hit_Anim`)

(event `Skill_Q`)

(event `OnHitReact`
  (params (Blocking :type Boolean))
  ;[1 1 1] Play hit react anim (includes block hit)
  (if (not Blocking)
    (`self.Hit_Anim`)
    (`MovementComponent.StopMovementImmediately` (`self.CharacterMovement`))
    (`self.OnChangeStates` true)
    (`KismetSystemLibrary.K2_SetTimer` self "RestoreInputAndStates" 0.5)
    (else
      (`self.Hit_Anim_Blocking`))))

(event `Skill_W`)

(event `/Game/BossAIToolkit/Blueprints/Interfaces/BI_CrowdControl.ReceiveCrowdControl`
  (params (ControlType :type "/Game/BossAIToolkit/Blueprints/Enums/E_CrowdControl Enum" :default "NewEnumerator0") (SourceLocation :type "Vector Structure") (Duration :type "Float (single-precision)"))
  (bind _bpc_statuseffects (`self.BPC_StatusEffects`))
  ;[1 1 1] Player receives crowd control status
  (if (`|EnumInequality` ControlType "NewEnumerator0")
    (if (`self.bCanBeDamaged`)
      (`/Engine/EditorBlueprintResources/StandardMacros.IsValid` _bpc_statuseffects
        (:`Is Valid`
          (bind _success (`/Game/BossAIToolkit/Blueprints/BPC_StatusEffects.ApplyCrowdControl` _bpc_statuseffects ControlType SourceLocation Duration))
          (if _success
            (`self.OnChangeStates` true ControlType)
            (`KismetSystemLibrary.K2_SetTimer` self "RestoreInputAndStates" Duration)))))))

(event `/Game/BossAIToolkit/Blueprints/Interfaces/BI_CrowdControl.ReceiveDebuff`
  (params (Type :type "/Game/BossAIToolkit/Blueprints/Enums/E_BossDebuffs Enum" :default "NewEnumerator1") (Duration :type "Float (single-precision)") (Damage :type "Float (single-precision)"))
  (bind _bpc_statuseffects (`self.BPC_StatusEffects`))
  ;[1 1 1] Player receives a debuff
  (`/Engine/EditorBlueprintResources/StandardMacros.IsValid` _bpc_statuseffects
    (:`Is Valid`
      (`/Game/BossAIToolkit/Blueprints/BPC_StatusEffects.ApplyDebuff` _bpc_statuseffects Type Duration Damage))))

(event `Server_OnAttack`
  (params (AttackType :type "/Game/BossAIToolkit/Blueprints/Enums/E_HitType Enum" :default "NewEnumerator1"))
  ;[1 1 1] Attacking
  (`self.OnAttack` AttackType (select `bool` (> (`self.Stamina`) 0.0) :`false` 0.7 :`true` 1.0 :!type "Float (single-precision)"))
  (`self.OnSprint` false))

(event `MouseAutoLockOn`
  (params (CharacterMovement :type "CharacterMovementComponent Object Reference") (YawMouse :type "Float (double-precision)") (NewParam :type "PlayerController Object Reference"))
  (`SceneComponent.K2_SetWorldRotation` (`MovementComponent.UpdatedPrimitive` CharacterMovement) (`KismetMathLibrary.MakeRotator` 0.0 0.0 YawMouse) false false))

(event `OnAttack`
  (params (AttackType :type "/Game/BossAIToolkit/Blueprints/Enums/E_HitType Enum" :default "NewEnumerator1") (PlayRate :type "Float (double-precision)"))
  ;[1 1 1] Attacking
  (set `self.AttackType` AttackType)
  (set `self.IsAttacking` true)
  (`CharacterMovementComponent.DisableMovement` (`self.CharacterMovement`))
  (bind _notifyname (`|PlayMontage` (`self.Mesh`) (select `/Game/BossAIToolkit/Blueprints/Enums/E_HitType` (`self.AttackType`) :`NewEnumerator1` (select `int` (`self.ComboIndex`) :`0` "/Game/BossAIToolkit/Demo/Mannequin/Animations/AM_Attack_01.AM_Attack_01" :`1` "/Game/BossAIToolkit/Demo/Mannequin/Animations/AM_Attack_02.AM_Attack_02" :`2` "/Game/BossAIToolkit/Demo/Mannequin/Animations/AM_Attack_03.AM_Attack_03" :!type "AnimMontage Object Reference") :`NewEnumerator2` "/Game/BossAIToolkit/Demo/Mannequin/Animations/AM_HeavyAttack.AM_HeavyAttack") PlayRate)
    (:`then`
      (`/Engine/EditorBlueprintResources/ActorMacros.Switch Has Authority`
        (:`Authority`
          (`self.ConsumeStamina` (select `/Game/BossAIToolkit/Blueprints/Enums/E_HitType` (`self.AttackType`) :`NewEnumerator1` 10.0 :`NewEnumerator2` 15.0 :!type "Float (single-precision)"))
          (`KismetSystemLibrary.Delay` 0.2)
          (`/Game/BossAIToolkit/Blueprints/Misc/BFL_Misc.SendAttackMessage` (`self.K2_GetActorLocation`) self))))
    (:`OnCompleted`
      (set `self.ComboIndex` 0)
      (set `self.IsAttacking` false)
      (`CharacterMovementComponent.SetMovementMode` (`self.CharacterMovement`) "MOVE_Walking" 0 :!label _label)
      (`/Engine/EditorBlueprintResources/ActorMacros.Switch Has Authority`
        (:`Authority`
          (if (`|EnumEquality` (`self.ActionState`) "NewEnumerator0")
            (`KismetSystemLibrary.K2_SetTimer` null "RegenStamina" 1.0 true)))))
    (:`OnInterrupted`
      (goto _label))
    (:`OnNotifyBegin`
      (`/Engine/EditorBlueprintResources/ActorMacros.Switch Has Authority`
        (:`Authority`
          (switch `name` _notifyname
            (:`Damage`
              (set `self.CanDealDamage` true))
            (:`Combo`
              (set `self.ComboIndex` (mod (+ (`self.ComboIndex`) 1) 3))
              (set `self.IsAttacking` false))))))
    (:`OnNotifyEnd`
      (`/Engine/EditorBlueprintResources/ActorMacros.Switch Has Authority`
        (:`Authority`
          (switch `name` _notifyname
            (:`Damage`
              (set `self.CanDealDamage` false)
              (`KismetArrayLibrary.Array_Clear` (`self.DamagedActors`)))))))))

(event `dash_server`
  (params (`타깃` :type "CharacterMovementComponent Object Reference") (`타깃2` :type "SceneComponent Object Reference"))
  (set `CharacterMovementComponent.MaxAcceleration` 9999.0 `타깃`)
  (set `CharacterMovementComponent.MaxWalkSpeed` 2000.0 `타깃`)
  (`Timeline|타임라인_0` :!via `PlayFromStart`
    (:`Update`
      (`self.AddMovementInput` (`SceneComponent.GetForwardVector` `타깃2`)))
    (:`Finished`
      (set `CharacterMovementComponent.MaxAcceleration` 600.0 `타깃`)
      (set `CharacterMovementComponent.MaxWalkSpeed` 600.0 `타깃`))))

(event `Server_OnLockOnTarget`
  (params (Reset :type Boolean))
  ;[1 1 1] Lock on target
  (`self.OnLockOnTarget` Reset))

(event `InputAction|Dash`
  (params (Key :type "Key Structure"))
  (bind _charactermovement (`self.CharacterMovement`))
  (bind _charactermovement_2 (`self.CharacterMovement`))
  (bind _charactermovement_3 (`self.CharacterMovement`))
  (bind _charactermovement_4 (`self.CharacterMovement`))
  (:`Pressed`
    (if (`self.CanDush?`)
      (set `self.CanDush?` false)
      (bind _returnvalue (`|SpawnActorFromClass` "/Game/_Dev/Stage2/Char/skill/Ability_Dash.Ability_Dash_C" (`self.GetTransform`) "Undefined" "OverrideRootScale" null null))
      (`/Game/_Dev/Stage2/Char/skill/Ability_Dash.ApplyDash` _returnvalue)
      (`/Engine/EditorBlueprintResources/ActorMacros.Switch Has Authority`
        (:`Authority`
          (set `CharacterMovementComponent.MaxAcceleration` 9999.0 _charactermovement_4)
          (set `CharacterMovementComponent.MaxWalkSpeed` 2000.0 _charactermovement_4)
          (`Timeline|Dash` :!via `PlayFromStart`
            (:`Update`
              (`self.AddMovementInput` (`SceneComponent.GetForwardVector` (`self.CapsuleComponent`))))
            (:`Finished`
              (set `CharacterMovementComponent.MaxAcceleration` 600.0 _charactermovement_3)
              (set `CharacterMovementComponent.MaxWalkSpeed` 600.0 _charactermovement_3))))
        (:`Remote`
          (`self.dash_server` (`self.CharacterMovement`) (`self.CapsuleComponent`))
          (set `CharacterMovementComponent.MaxAcceleration` 9999.0 _charactermovement_2)
          (set `CharacterMovementComponent.MaxWalkSpeed` 2000.0 _charactermovement_2)
          (`Timeline|타임라인_1` :!via `PlayFromStart`
            (:`Update`
              (`self.AddMovementInput` (`SceneComponent.GetForwardVector` (`self.CapsuleComponent`))))
            (:`Finished`
              (set `CharacterMovementComponent.MaxAcceleration` 600.0 _charactermovement)
              (set `CharacterMovementComponent.MaxWalkSpeed` 600.0 _charactermovement))))))))

(event `OnLockOnTarget`
  (params (Reset :type Boolean))
  (bind _charactermovement (`self.CharacterMovement`))
  (bind _lockontarget (`self.LockOnTarget`))
  (bind _charactermovement_2 (`self.CharacterMovement`))
  (bind _lockontarget_2 (`self.LockOnTarget`))
  ;[1 1 1] Lock on target
  (if (not Reset)
    (`/Engine/EditorBlueprintResources/StandardMacros.IsValid` _lockontarget
      (:`Is Valid`
        (message `/Game/BossAIToolkit/Blueprints/Interfaces/BI_BossAI.SetLockOnVisibility` _lockontarget false))
      (:`Is Not Valid`
        _))
    (bind _outactors (`GameplayStatics.GetAllActorsOfClass` "/Game/BossAIToolkit/Blueprints/BP_Boss_Base.BP_Boss_Base_C"))
    (bind _output_get (set `self.LockOnTarget` (`|GetArrayItem` _outactors (`self.LockOnIndex`))))
    (`/Engine/EditorBlueprintResources/StandardMacros.IsValid` _output_get
      (:`Is Valid`
        (set `self.IsLockedOn` true)
        (message `/Game/BossAIToolkit/Blueprints/Interfaces/BI_BossAI.SetLockOnVisibility` (`self.LockOnTarget`) true)
        (`/Engine/EditorBlueprintResources/StandardMacros.IncrementInt` (`self.LockOnIndex`)
          (:`  `
            (set `CharacterMovementComponent.bUseControllerDesiredRotation` true _charactermovement_2)
            (set `CharacterMovementComponent.bOrientRotationToMovement` false _charactermovement_2))))
      (:`Is Not Valid`
        (set `self.IsLockedOn` false :!label _label_2)
        (set `self.LockOnIndex` 0)
        (set `CharacterMovementComponent.bUseControllerDesiredRotation` true _charactermovement)
        (set `CharacterMovementComponent.bOrientRotationToMovement` true _charactermovement)))
    (else
      (`/Engine/EditorBlueprintResources/StandardMacros.IsValid` _lockontarget_2
        (:`Is Valid`
          (message `/Game/BossAIToolkit/Blueprints/Interfaces/BI_BossAI.SetLockOnVisibility` _lockontarget_2 false)
          (set `self.LockOnTarget` null)
          (goto _label_2))
        (:`Is Not Valid`
          (goto _label_2))))))

(event `Server_OnSetTargetRotation`
  (params (NewRotation :type "Rotator Structure"))
  ;[1 1 1] Set target rotation
  (set `self.TargetRotation` NewRotation))

(event `Server_OnDodge`
  ;[1 1 1] Dodging
  (`self.OnDodge`)
  (`self.OnSprint` false))

(event `OnDodge`
  (bind _charactermovement (`self.CharacterMovement`))
  (bind _charactermovement_2 (`self.CharacterMovement`))
  ;[1 1 1] Dodging
  (`/Engine/EditorBlueprintResources/ActorMacros.Switch Has Authority`
    (:`Authority`
      (set `self.ActionState` "NewEnumerator3")
      (`self.ConsumeStamina` 10.0))
    (:`Remote`
      _))
  (set `CharacterMovementComponent.bUseControllerDesiredRotation` false _charactermovement)
  (set `CharacterMovementComponent.bOrientRotationToMovement` true _charactermovement)
  ;;[1 1 1] Dodge Montage has a notify that disables damage taking for this Player
  (`|PlayMontage` (`self.Mesh`) "/Game/BossAIToolkit/Demo/Mannequin/Animations/AM_DodgeRoll.AM_DodgeRoll"
    (:`OnCompleted`
      _)
    (:`OnInterrupted`
      _))
  (set `CharacterMovementComponent.bUseControllerDesiredRotation` true _charactermovement_2)
  (set `CharacterMovementComponent.bOrientRotationToMovement` (not (`self.IsLockedOn`)) _charactermovement_2)
  (`CharacterMovementComponent.SetMovementMode` (`self.CharacterMovement`) "MOVE_Walking" 0)
  (`/Engine/EditorBlueprintResources/ActorMacros.Switch Has Authority`
    (:`Authority`
      (set `self.ActionState` "NewEnumerator0")
      (`KismetSystemLibrary.K2_SetTimer` null "RegenStamina" 1.0 true))))

(event `Server_StartBlock`
  ;[1 1 1] Blocking
  (set `self.ActionState` "NewEnumerator2")
  (`KismetSystemLibrary.K2_ClearTimer` null "RegenStamina")
  (`self.OnSprint` false))

(event `Server_EndBlock`
  ;[1 1 1] Blocking
  (set `self.ActionState` "NewEnumerator0")
  (set `self.BlockOnCooldown` true)
  (if (`|EnumEquality` (`self.ActionState`) "NewEnumerator0")
    (`KismetSystemLibrary.K2_SetTimer` null "RegenStamina" 1.0 true)
    (`KismetSystemLibrary.Delay` 0.25)
    (set `self.BlockOnCooldown` false)))

(event `OnChangeStates`
  (params (StopInput :type Boolean) (NewState :type "/Game/BossAIToolkit/Blueprints/Enums/E_CrowdControl Enum" :default "NewEnumerator0"))
  ;[1 1 1] Change crowd control and input states
  (if StopInput
    (set `self.CrowdControlState` NewState)
    (set `self.IsAttacking` false)
    (set `self.ComboIndex` 0)
    (`self.OnChangeInputs` true)
    (else
      (set `self.CrowdControlState` "NewEnumerator0")
      (`self.OnChangeInputs` false))))

(event `OnChangeInputs`
  (params (StopInput :type Boolean))
  ;[1 1 1] Change movement and collision based on input state
  (if StopInput
    (`self.DisableInput` (`self.ControllerRef`))
    (`CharacterMovementComponent.SetMovementMode` (`self.CharacterMovement`) "MOVE_Walking" 0)
    (`PrimitiveComponent.SetCollisionResponseToChannel` (`self.CapsuleComponent`) "ECC_Pawn" "ECR_Ignore")
    (else
      (`self.EnableInput` (`self.ControllerRef`))
      (`PrimitiveComponent.SetCollisionResponseToChannel` (`self.CapsuleComponent`) "ECC_Pawn" "ECR_Block"))))

(event `OnSprint`
  (params (NewSprint :type Boolean))
  ;[1 1 1] Sprint player
  (bind _output_get (set `self.IsSprinting` NewSprint))
  (set `CharacterMovementComponent.MaxWalkSpeed` (select `bool` _output_get :`false` 375.0 :`true` 600.0 :!type "Float (single-precision)") (`self.CharacterMovement`))
  (if (and (`self.IsSprinting`) (`self.IsLockedOn`))
    (`self.OnLockOnTarget` true)))

(fn `Attack Auto Mouse Lock On`
  (bind _yaw (`self.Set Mouse Auto Lock On Yaw`))
  (set `self.Yaw` _yaw)
  (`/Engine/EditorBlueprintResources/ActorMacros.Switch Has Authority`
    (:`Authority`
      (`SceneComponent.K2_SetWorldRotation` (`MovementComponent.UpdatedPrimitive` (`self.CharacterMovement`)) (`KismetMathLibrary.MakeRotator` 0.0 0.0 (`self.Yaw`)) false false))
    (:`Remote`
      (`self.MouseAutoLockOn` (`self.CharacterMovement`) (`self.Yaw`))
      (`SceneComponent.K2_SetWorldRotation` (`MovementComponent.UpdatedPrimitive` (`self.CharacterMovement`)) (`KismetMathLibrary.MakeRotator` 0.0 0.0 (`self.Yaw`)) false false))))

(fn `CheckBlock`
  (params (HitFrom :type "Vector Structure"))
  (returns (Blocked :type Boolean))
  (bind (_returnvalue_roll _returnvalue_pitch _returnvalue_yaw) (`KismetMathLibrary.BreakRotator` (`KismetMathLibrary.NormalizedDeltaRotator` (`self.K2_GetActorRotation`) (`KismetMathLibrary.FindLookAtRotation` (`self.K2_GetActorLocation`) HitFrom))))
  (return (and (`|EnumEquality` (`self.ActionState`) "NewEnumerator2") (< (`KismetMathLibrary.Abs` _returnvalue_yaw) (`self.BlockingAngle`)))))

(fn `ConsumeStamina`
  (params (StaminaDamage :type "Float (double-precision)"))
  (returns (ReturnValue :type "Float (double-precision)"))
  (bind _output_get (set `self.Stamina` (`KismetMathLibrary.FClamp` (- (`self.Stamina`) StaminaDamage) 0.0 (`self.MaxStamina`))))
  (`KismetSystemLibrary.K2_ClearTimer` null "RegenStamina")
  (return _output_get))

(fn `GetAbilityInfo`
  (returns (ReturnValue :type "/Game/BossAIToolkit/Blueprints/Structs/F_BossAbility Structure"))
  (return))

(fn `GetCrowdControlState`
  (returns (CurrentState :type "/Game/BossAIToolkit/Blueprints/Enums/E_CrowdControl Enum"))
  (return (`self.CrowdControlState`)))

(fn `GetPriorityScore`
  (params (Querier :type "Actor Object Reference") (IsEnemy :type Boolean))
  (returns (Score :type "Float (double-precision)"))
  (return (`KismetMathLibrary.MapRangeUnclamped` (`self.GetDistanceTo` Querier self) 0.0 5000.0 100.0 1.0)))

(fn `GetStaggerInfo`
  (returns (PostureDamage :type "Float (double-precision)") (HitType :type "/Game/BossAIToolkit/Blueprints/Enums/E_HitType Enum"))
  (bind _attacktype (`self.AttackType`))
  (return (select `/Game/BossAIToolkit/Blueprints/Enums/E_HitType` _attacktype :`NewEnumerator1` 8.0 :`NewEnumerator2` 15.0 :!type "Float (single-precision)") _attacktype))

(fn `GetStatusEffectInfo`
  (returns (Duration :type "Float (double-precision)") (Damage :type "Float (double-precision)") (CrowdControl :type "/Game/BossAIToolkit/Blueprints/Enums/E_CrowdControl Enum") (CC_Duration :type "Float (double-precision)"))
  (return 0.0 0.0 "NewEnumerator0" 0.0))

(fn `OnRep_CriticalShield`
  (bind _criticalshield (`self.CriticalShield`))
  (if (== _criticalshield 0)
    _
    (elif (== _criticalshield 1)
      (`ActorComponent.SetActive` (`self.ParticleSystem_Buff1`) true false)
      (else
        (`ActorComponent.SetActive` (`self.ParticleSystem_Buff1`) false false)
        (`ActorComponent.SetActive` (`self.ParticleSystem_Buff2`) true false)))))

(fn `RegenStamina`
  (set `self.Stamina` (`KismetMathLibrary.FClamp` (+ (`self.Stamina`) (`self.StaminaRegenPassive`)) 0.0 (`self.MaxStamina`)))
  (return))

(fn `RestoreInputAndStates`
  (`self.OnChangeStates` false))

(fn `Set Mouse Auto Lock On Yaw`
  (returns (Yaw :type "Float (double-precision)"))
  (bind _returnvalue (`KismetMathLibrary.GetDirectionUnitVector` (`self.K2_GetActorLocation`) (`.Location` (`GameplayStatics.BreakHitResult` (`PlayerController.GetHitResultUnderCursorByChannel` (`GameplayStatics.GetPlayerController` 0) "TraceTypeQuery1" true)))))
  (`KismetSystemLibrary.PrintString` (`KismetStringLibrary.Concat_StrStr` "방향 : " (`KismetStringLibrary.Conv_DoubleToString` (.z _returnvalue))))
  (return (.yaw (`KismetMathLibrary.Conv_VectorToRotator` _returnvalue))))

(fn `TakeDamage`
  (params (Damage :type "Float (double-precision)") (DamageType :type "DamageType Object Reference") (HitFrom :type "Vector Structure (by ref)") (Blocked :type Boolean))
  (bind _blocked (`local.Blocked`))
  ;[1 1 1] Decrease player health. NOTE: Process Damage has already reduced the damage if it was blocked
  (bind _output_get (set `self.Health` (- (`self.Health`) Damage)))
  ;[1 1 1] If health is 0, then player is dead
  (if (<= _output_get 0.0)
    (`self.OnDeath`)
    (else
      ;[1 1 1] If not crowd controlled and DamagType is not from status effect, then play hit react anim
      (if (and (`|EnumEquality` (`self.CrowdControlState`) "NewEnumerator0") (!= (`GameplayStatics.GetObjectClass` (`local.DamageType`)) "/Game/BossAIToolkit/Blueprints/DamageTypes/BP_DamageType_Overtime.BP_DamageType_Overtime_C"))
        (`self.OnHitReact` _blocked)
        ;[1 1 1] If attack was blocked, then consume stamina based on damage. If stamina is 0, then stop blocking
        (if _blocked
          (bind _returnvalue (`self.ConsumeStamina` (* (`local.Damage`) 0.3)))
          (if (<= _returnvalue 0.0)
            (`self.Server_EndBlock`)))))))

(fn `UserConstructionScript`)