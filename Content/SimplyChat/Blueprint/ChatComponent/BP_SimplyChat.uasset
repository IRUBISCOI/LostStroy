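; Chat component that gives the local player's owning pawn or controller a SimplyChat widget.
; On startup it creates or reuses the widget, adds it to the viewport and posts a welcome using the GameInstance player name.
; ServerUpdaterChat fans each message out through every BPI_SimplyChat actor's component to OwnClientUpdaterChat, which updates that widget.
; A helper moves keyboard focus to the chat input.
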(event `OwnClient StartUP UI`
  ;[0.5067 1 0.1729] Create chat UI on start
  (if (`self.OwnValid?`)
    (`self.Create UI`)))

(event `OwnClient Updater Chat`
  (params (Message :type "/Game/SimplyChat/Blueprint/Structures/S_SimplyChat Structure"))
  ;[0.1063 0.2664 1] Update chat for own client (Sended message and check is valid chat)
  (bind _simplychat_ref (`self.SimplyChat Ref`)
    (:`then`
      (`/Game/SimplyChat/Blueprint/UI/WBP_SimplyChat_body.UpdateChat` _simplychat_ref Message))
    (:`else`)))

(event `Server Updater Chat`
  (params (Message :type "/Game/SimplyChat/Blueprint/Structures/S_SimplyChat Structure"))
  ;[0.02034 0.9702 1] Send message for all
  (bind _outactors (`GameplayStatics.GetAllActorsWithInterface` "/Game/SimplyChat/Blueprint/ChatComponent/BPI_SimplyChat.BPI_SimplyChat_C"))
  (for _array_element _outactors
    (bind _simplychat_ref (message `/Game/SimplyChat/Blueprint/ChatComponent/BPI_SimplyChat.Get SimplyChat` _array_element))
    (`self.OwnClient Updater Chat` _simplychat_ref Message)))

(fn `Create UI`
  (bind _simplychat_ref (`self.SimplyChat Ref`)
    (:`then`
      (if (not (`Widget.IsInViewport` _simplychat_ref))
        (`UserWidget.AddToViewport` _simplychat_ref 0 :!label _label)
        (bind _asgame_instance (cast `/Game/_DevelopersFolder/GameInstance` (`GameplayStatics.GetGameInstance`)))
        (`self.OwnClient Updater Chat` (make `/Game/SimplyChat/Blueprint/Structures/S_SimplyChat` "" (`KismetTextLibrary.Conv_TextToString` (`|FormatText` "Welcome back, {name}!  \nPress ENTER for start typing." (`/Game/_DevelopersFolder/GameInstance.PlayerName` _asgame_instance))) "NewEnumerator4"))))
    (:`else`
      (bind _returnvalue (`|CreateWidget` "/Game/SimplyChat/Blueprint/UI/WBP_SimplyChat_body.WBP_SimplyChat_body_C" null (`self.GetOwner`)))
      (set `self.SimplyChat Ref` _returnvalue)
      (goto _label))))

(fn `Focus Keyboard`
  (bind _simplychat_ref (`self.SimplyChat Ref`)
    (:`then`
      (`Widget.SetKeyboardFocus` (`/Game/SimplyChat/Blueprint/UI/WBP_SimplyChat_body.Input` _simplychat_ref))
      (`/Game/SimplyChat/Blueprint/UI/WBP_SimplyChat_body.Focus Chat` _simplychat_ref))
    (:`else`)))

(fn `OwnValid?`
  (returns (`Var Own` :type Boolean))
  (bind _returnvalue (`self.GetOwner`))
  (return (or (== (`GameplayStatics.GetPlayerPawn` 0) _returnvalue) (== (`GameplayStatics.GetPlayerController` 0) _returnvalue))))