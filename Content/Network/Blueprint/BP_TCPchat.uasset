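; TCP chat client that connects to a hard-coded server address and port on BeginPlay.
; Connection callbacks store or clear the server socket ID; incoming messages are decoded as strings, followed by a debug print that is not wired to the decoded text.
; TCPSendMessage and TCPUserName send text as bytes over that socket, calling the disconnect handler and then setting the ID to 0 if sending fails.
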(event `self.ReceiveBeginPlay`
  (`self.Connect` "172.16.2.253" 4949 (delegate `TCPDisconnected`) (delegate `TCPConnected`) (delegate `OnRecvMessage`)))

(event `TCPDisconnected`
  (params (ConnectionId :type Integer))
  (set `self.ServerSocket` -1))

(event `TCPConnected`
  (params (ConnectionId :type Integer))
  (set `self.ServerSocket` ConnectionId))

(event `OnRecvMessage`
  (params (ConnectionId :type Integer) (Message :type "Array of Byte (by ref)"))
  (`self.Message_ReadString` Message (`KismetArrayLibrary.Array_Length` Message))
  (`KismetSystemLibrary.PrintString` "Hello" true true (struct :`R` 0.842658 :`G` 1.0 :`B` 0.281627 :`A` 1.0)))

(fn `TCPSendMessage`
  (params (Message :type String))
  (bind _serversocket (`self.ServerSocket`))
  (bind _returnvalue (`self.SendData` _serversocket (`self.Conv_StringToBytes` Message)))
  (if (not _returnvalue)
    (`self.TCPDisconnected` _serversocket)
    (set `self.ServerSocket` 0)))

(fn `TCPUserName`
  (params (UserName :type String))
  (bind _returnvalue (`self.SendData` (`self.ServerSocket`) (`self.Conv_StringToBytes` UserName)))
  (if (not _returnvalue)
    (`self.TCPDisconnected` 0)
    (set `self.ServerSocket` 0)))

(fn `UserConstructionScript`)