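; YDYGameState is a networked game state that runs a boss gimmick involving a replicated rock-paper-scissors value.
; Shortly after BeginPlay it starts the gimmick through YDYHUD.
; CheckGimmic calls GimmicStart on the first player controller, then ReleaseGimmic if GimmicProblem matches BossGimmicCheck; an inner condition is hardcoded true.
; The RandRPS OnRep copies the value to the first player character, with debug prints throughout.
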(event `self.ReceiveBeginPlay`
  ;[1 1 1] 기믹 이벤트 발생
  (`KismetSystemLibrary.PrintString` "gimic start")
  (`KismetSystemLibrary.Delay` 0.2)
  (`self.GimmicPlay`))

(event `CheckGimmic`
  (bind _asbp_pc_tpc (cast `/Game/SimplyChat/DEMO/ThirdPersonBP/Blueprints/BP_PC_TPC` (`GameplayStatics.GetPlayerController` 0)))
  (`/Game/SimplyChat/DEMO/ThirdPersonBP/Blueprints/BP_PC_TPC.GimmicStart` _asbp_pc_tpc)
  (if (`KismetStringLibrary.EqualEqual_StrStr` (`self.GimmicProblem`) (`self.BossGimmicCheck`))
    (if true
      (`KismetSystemLibrary.PrintString` "기믹 해제")
      (`/Game/SimplyChat/DEMO/ThirdPersonBP/Blueprints/BP_PC_TPC.ReleaseGimmic` _asbp_pc_tpc)
      (else
        (`KismetSystemLibrary.PrintString` "아직 ")))
    (else
      (`KismetSystemLibrary.PrintString` "fail"))))

(fn `GimmicPlay`
  (`KismetSystemLibrary.PrintString` "기믹 시작" true true (struct :`R` 1.0 :`G` 0.208059 :`B` 0.227956 :`A` 1.0))
  (bind _asydyhud (cast `/Game/Network/Level/YDYHUD` (`PlayerController.GetHUD` (`GameplayStatics.GetPlayerController` 0))))
  (`/Game/Network/Level/YDYHUD.GimmicPlay` _asydyhud))

(fn `OnRep_Rand_RPS`
  (bind _asbp_player_base (cast `/Game/_Dev/Stage2/Char/BP_Player_Base` (`GameplayStatics.GetPlayerCharacter` 0)))
  (bind _output_get (set `/Game/_Dev/Stage2/Char/BP_Player_Base.RandomRPS` (`self.Rand_RPS`) _asbp_player_base))
  (`KismetSystemLibrary.PrintString` (`KismetStringLibrary.Concat_StrStr` "RPS : " (`KismetStringLibrary.Conv_IntToString` _output_get))))

(fn `UserConstructionScript`)