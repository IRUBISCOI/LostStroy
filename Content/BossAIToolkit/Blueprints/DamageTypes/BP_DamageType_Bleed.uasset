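; BP_DamageType_Bleed is a Boss AI Toolkit damage type that adds a bleed effect to unblocked hits.
; ProcessDamage reads status effect info from the damage causer, then sends debuff and crowd-control messages to a valid damaged actor, using the causer's location as the control source.
; Blocked hits apply no effects and return zero damage, while unblocked hits return the incoming damage unchanged.
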(fn `ProcessDamage`
  (params (DamagedActor :type "Actor Object Reference") (Damage :type "Float (double-precision)") (Blocked :type Boolean) (DamageCauser :type "Actor Object Reference"))
  (returns (NewDamage :type "Float (double-precision)"))
  (bind _damagedactor (`local.DamagedActor`))
  (`/Engine/EditorBlueprintResources/StandardMacros.IsValid` DamagedActor
    (:`Is Valid`
      (if (not Blocked)
        (bind (_duration _damage _crowdcontrol _cc_duration) (message `/Game/BossAIToolkit/Blueprints/Interfaces/BI_Ability.GetStatusEffectInfo` (`local.DamageCauser`)))
        (message `/Game/BossAIToolkit/Blueprints/Interfaces/BI_CrowdControl.ReceiveDebuff` _damagedactor "NewEnumerator1" _duration _damage)
        (message `/Game/BossAIToolkit/Blueprints/Interfaces/BI_CrowdControl.ReceiveCrowdControl` _damagedactor _crowdcontrol (`Actor.K2_GetActorLocation` (`local.DamageCauser`)) _cc_duration)))
    (:`Is Not Valid`
      _))
  (return (select `bool` (`local.Blocked`) :`false` (`local.Damage`))))