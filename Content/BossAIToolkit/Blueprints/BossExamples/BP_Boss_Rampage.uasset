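; Example Rampage boss Blueprint from a boss AI toolkit, inheriting its startup, tick and construction behavior from a parent class.
; Its own logic is the DelayDestroy event, which disables collision on the capsule, mesh and both arm hitboxes.
; The event then prints an on-screen debug message and destroys the actor after a fixed delay.
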(event `self.ReceiveBeginPlay`
  (`parent.ReceiveBeginPlay`))

(event `self.DelayDestroy`
  (`PrimitiveComponent.SetCollisionEnabled` (`self.CapsuleComponent`) "NoCollision")
  (`PrimitiveComponent.SetCollisionEnabled` (`self.Mesh`) "NoCollision")
  (`PrimitiveComponent.SetCollisionEnabled` (`self.Hitbox_ArmR`) "NoCollision")
  (`PrimitiveComponent.SetCollisionEnabled` (`self.Hitbox_ArmL`) "NoCollision")
  (`KismetSystemLibrary.PrintString` "Hello" true true (struct :`R` 0.021328 :`B` 1.0 :`A` 1.0) 10.0)
  (`KismetSystemLibrary.Delay` 10.0)
  (`self.K2_DestroyActor`))

(event `self.ReceiveTick`
  (params (DeltaSeconds :type "Float (single-precision)"))
  (`parent.ReceiveTick` DeltaSeconds))

(fn `UserConstructionScript`
  (`parent.UserConstructionScript`))