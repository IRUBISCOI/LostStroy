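; Boss charge ability that rushes the boss in a straight line toward the target over the ability's max targeting distance.
; On begin play it faces the target, fixes the end point and shows a beam telegraph sized from the ability modifier.
; Execution removes the telegraph and drives a swept location lerp with a timeline scaled to the given duration.
; During the damage window, Tick damages hits from custom hitboxes, or a box trace around the boss when none exist.
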(event `self.ReceiveBeginPlay`
  (bind (_hitboxsize_x _hitboxsize_y _hitboxsize_z) (`KismetMathLibrary.BreakVector` (`self.HitboxSize`)))
  (bind _returnvalue (`self.K2_GetActorLocation` (`self.BossRef`)))
  (bind _returnvalue_2 (`self.K2_GetActorLocation` (`self.TargetActor`)))
  (bind (_returnvalue_roll _returnvalue_pitch _returnvalue_yaw) (`KismetMathLibrary.BreakRotator` (`KismetMathLibrary.FindLookAtRotation` _returnvalue _returnvalue_2)))
  (`parent.ReceiveBeginPlay`)
  (set `self.Distance` (`.MaxDistance_10_DB850DAD4E3F0E316EDA76876616FD4B` (break `/Game/BossAIToolkit/Blueprints/Structs/F_BossAbilityTargeting` (`.Targeting_67_C3E0562A42DA13AB69A88191173DAD2E` (break `/Game/BossAIToolkit/Blueprints/Structs/F_BossAbility` (`self.AbilityInfo`))))))
  (`self.ForceRotateAI` _returnvalue_2)
  (bind _output_get (set `self.InitialLocation` _returnvalue))
  (set `self.FinalLocation` (+ _output_get (* (`KismetMathLibrary.GetForwardVector` (`KismetMathLibrary.MakeRotator` 0.0 0.0 _returnvalue_yaw)) (`self.Distance`))))
  (set `self.HitboxSize` (`.Modifier_68_9F6259774C70A5FB7DE538BB3C951747` (break `/Game/BossAIToolkit/Blueprints/Structs/F_BossAbility` (`self.AbilityInfo`))))
  (`self.TelegraphBeam` (+ (`self.Distance`) _hitboxsize_x) (* _hitboxsize_y 2.0) _hitboxsize_z (- (`self.InitialLocation`) (0.0 0.0 50.0)) (`self.FinalLocation`)))

(event `self.OnBeginDamage`
  (params (Duration :type "Float (single-precision)"))
  (set `self.CanDealDamage` true))

(event `self.OnEndDamage`
  (set `self.CanDealDamage` false)
  (`KismetArrayLibrary.Array_Clear` (`self.DamagedActors`))
  (`self.ResetRotation`))

(event `self.OnExecute`
  (params (Duration :type "Float (single-precision)"))
  (`AIController.K2_SetFocus` (`AIBlueprintHelperLibrary.GetAIController` (`self.BossRef`)) null)
  (`self.RemoveTelegraph`)
  (`TimelineComponent.SetPlayRate` (`self.Charge_Timeline`) (/ 1.0 Duration))
  (bind (_direction _alpha) (`Timeline|Charge_Timeline` :!via `PlayFromStart`)
    (:`Update`
      (`self.K2_SetActorLocation` (`self.BossRef`) (`KismetMathLibrary.VLerp` (`self.InitialLocation`) (`self.FinalLocation`) _alpha) true false))))

(event `self.ReceiveTick`
  (params (DeltaSeconds :type "Float (single-precision)"))
  (bind _bossref (`self.BossRef`))
  (bind _returnvalue (`self.K2_GetActorLocation` _bossref))
  (if (`self.CanDealDamage`)
    (if (== (`KismetArrayLibrary.Array_Length` (`self.Hitboxes`)) 0)
      (bind _outhits (`KismetSystemLibrary.BoxTraceMultiForObjects` _returnvalue (+ _returnvalue (0.0 0.0 1.0)) (`self.HitboxSize`) (`self.K2_GetActorRotation` _bossref) (`|MakeArray` "ObjectTypeQuery3" :!type "EObjectTypeQuery Enum") false (`|MakeArray` _bossref :!type "Actor Object Reference") (`self.GetDebugType`)))
      (for _array_element _outhits
        (`self.ApplyAbilityDamage` (`.HitActor` (`GameplayStatics.BreakHitResult` _array_element)) (`self.K2_GetActorLocation` (`self.BossRef`))))
      (else
        (bind _outactors (`self.TraceHitbox`))
        (for _array_element_2 _outactors
          (`self.ApplyAbilityDamage` _array_element_2 (`self.K2_GetActorLocation` (`self.BossRef`))))))))

(fn `UserConstructionScript`
  (`parent.UserConstructionScript`))