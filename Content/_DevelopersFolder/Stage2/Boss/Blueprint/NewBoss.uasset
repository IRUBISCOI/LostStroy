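; Stage 2 boss character that switches into an orb-summon gimmick phase, driven by the BossBehavior component's phase changes.
; In phase index 1 it teleports to the center locator, hides its mesh, disables collision and swaps to poison materials.
; While an ability plays in that phase, Tick stops the AI brain and movement.
; Other phases restart AI logic and restore visibility, body and sword collision, and fire materials.
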(event `self.ReceiveTick`
  (params (DeltaSeconds :type "Float (single-precision)"))
  (`parent.ReceiveTick` DeltaSeconds)
  (if (== (`/Game/BossAIToolkit/Blueprints/BPC_Boss_Behavior.GetCurrentPhaseInfo` (`self.Boss Behavior`)) 1)
    (if (`/Game/BossAIToolkit/Blueprints/BPC_Boss_Behavior.IsPlayingAbility` (`self.Boss Behavior`))
      (`self.OnPlayingAbility`))))

(event `self.Boss Behavior.OnPhaseChange`
  (params (NewPhaseIndex :type Integer))
  (bind _controllerref (`self.ControllerRef`))
  ;[1 1 1] 내장 Phase 기능 + Visibility + Collision 기능
  (if (== (`/Game/BossAIToolkit/Blueprints/BPC_Boss_Behavior.GetCurrentPhaseInfo` (`self.Boss Behavior`)) 1)
    (`KismetSystemLibrary.PrintString` "구슬 소환!!!!" true true (struct :`R` 1.0 :`B` 0.396417 :`A` 1.0) 10.0)
    ;;[1 1 1] 보스 가운데로
    (bind _outactors (`GameplayStatics.GetAllActorsOfClass` "/Game/_DevelopersFolder/Stage2/Boss/Blueprint/BP_CenterLocator.BP_CenterLocator_C"))
    (`self.K2_SetActorLocation` self (`self.K2_GetActorLocation` (`|GetArrayItem` _outactors)) false true)
    (`SceneComponent.SetVisibility` (`self.Mesh`) false false)
    (`self.CollisionsOff`)
    (`self.SetMaterial`)
    (else
      (`/Engine/EditorBlueprintResources/StandardMacros.IsValid` _controllerref
        (:`Is Valid`
          (`BrainComponent.RestartLogic` (`AIController.BrainComponent` _controllerref))
          (`SceneComponent.SetVisibility` (`self.Mesh`) true false)
          (`self.CollisionsON`)
          (`self.SetMaterial2`))))))

(event `OnPlayingAbility`
  ;[1 1 1] 내장 Phase 기능 + Visibility + Collision 기능
  ;;[1 1 1] 스킬 쓸때, 로직 멈추기
  (set `self.Logic Stoped` (`self.Stop Logic and Mov`))
  (set `self.IsGimmickPassed` true))

(fn `CollisionsOff`
  (`PrimitiveComponent.SetCollisionEnabled` (`self.CapsuleComponent`) "NoCollision")
  (`PrimitiveComponent.SetCollisionEnabled` (`self.Mesh`) "NoCollision")
  (`PrimitiveComponent.SetCollisionEnabled` (`self.Katana`) "NoCollision")
  (`PrimitiveComponent.SetCollisionEnabled` (`self.Sword_L`) "NoCollision")
  (`PrimitiveComponent.SetCollisionEnabled` (`self.Sword_R`) "NoCollision"))

(fn `CollisionsON`
  (`PrimitiveComponent.SetCollisionEnabled` (`self.CapsuleComponent`) "QueryAndPhysics")
  (`PrimitiveComponent.SetCollisionEnabled` (`self.Mesh`) "QueryOnly")
  (`PrimitiveComponent.SetCollisionEnabled` (`self.Katana`) "NoCollision")
  (`PrimitiveComponent.SetCollisionEnabled` (`self.Sword_L`) "QueryOnly")
  (`PrimitiveComponent.SetCollisionEnabled` (`self.Sword_R`) "QueryOnly"))

(fn `IsHealthBelowX`
  (params (Percent :type "Float (double-precision)"))
  (returns (NewParam :type Boolean))
  (bind _boss_behavior (`self.Boss Behavior`))
  (return (< (`/Game/BossAIToolkit/Blueprints/BPC_Boss_Behavior.Health` _boss_behavior) (/ (* (`/Game/BossAIToolkit/Blueprints/BPC_Boss_Behavior.MaxHealth` _boss_behavior) Percent) 100.0))))

(fn `SetMaterial`
  (bind _mesh (`self.Mesh`))
  (`PrimitiveComponent.SetMaterial` _mesh 1 "/Game/InfinityBladeEffects/Effects/FX_Materials/Poison/M_JaggedRockPoison_MeshEmit_Lit_INST.M_JaggedRockPoison_MeshEmit_Lit_INST")
  (`PrimitiveComponent.SetMaterial` _mesh 2 "/Game/InfinityBladeEffects/Effects/FX_Materials/Poison/M_JaggedRockPoison_MeshEmit_Lit_INST.M_JaggedRockPoison_MeshEmit_Lit_INST"))

(fn `SetMaterial2`
  (bind _mesh (`self.Mesh`))
  (`PrimitiveComponent.SetMaterial` _mesh 1 "/Game/InfinityBladeEffects/Effects/FX_Materials/Fire/M_JaggedRockFire_MeshEmit_Lit.M_JaggedRockFire_MeshEmit_Lit")
  (`PrimitiveComponent.SetMaterial` _mesh 2 "/Game/InfinityBladeEffects/Effects/FX_Materials/Fire/M_JaggedRockFire_MeshEmit_Lit.M_JaggedRockFire_MeshEmit_Lit"))

(fn `Stop Logic and Mov`
  (returns (LogicStoped :type Boolean))
  (locals (NewLocalVar_0 :type Boolean :default true))
  (bind _controllerref (`self.ControllerRef`))
  ;[1 1 1] 체력 x% 이하 시,  정지
  (`/Engine/EditorBlueprintResources/StandardMacros.IsValid` _controllerref
    (:`Is Valid`
      (`BrainComponent.StopLogic` (`AIController.BrainComponent` _controllerref) "")
      (`Controller.StopMovement` _controllerref)
      (return true))))

(fn `UserConstructionScript`
  (`parent.UserConstructionScript`))