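; Stage 2 player controller that hosts the SimplyChat component for in-game text chat.
; The local controller starts the chat UI on BeginPlay, and Enter focuses the chat input.
; A game mode message event loops over the game mode's AllPC list, pushing the message with an empty sender name to each BP_PC_TPC's chat.
; Accessor functions expose the chat component and the player name stored in BP_GameInstance.
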(event `self.ReceiveBeginPlay`
  (if (`self.IsLocalPlayerController`)
    (`/Game/SimplyChat/Blueprint/ChatComponent/BP_SimplyChat.OwnClient StartUP UI` (`self.SimplyChat`))))

(event `Key|Enter`
  (params (Key :type "Key Structure"))
  (:`Pressed`
    (`/Game/SimplyChat/Blueprint/ChatComponent/BP_SimplyChat.Focus Keyboard` (`self.SimplyChat`))))

(event `Message from gamemode`
  (params (Message :type String) (Type :type "/Game/SimplyChat/Blueprint/Structures/E_SimplyChat Enum" :default "NewEnumerator0"))
  (bind _asbpc_gm_tpc (cast `/Game/SimplyChat/DEMO/ThirdPersonBP/Blueprints/BPC_GM_TPC` (`GameplayStatics.GetGameMode`)))
  (for _array_element (`/Game/SimplyChat/DEMO/ThirdPersonBP/Blueprints/BPC_GM_TPC.All PC` _asbpc_gm_tpc)
    (bind _asbp_pc_tpc (cast `/Game/SimplyChat/DEMO/ThirdPersonBP/Blueprints/BP_PC_TPC` _array_element))
    (`/Game/SimplyChat/Blueprint/ChatComponent/BP_SimplyChat.OwnClient Updater Chat` (`/Game/SimplyChat/DEMO/ThirdPersonBP/Blueprints/BP_PC_TPC.SimplyChat` _asbp_pc_tpc) (make `/Game/SimplyChat/Blueprint/Structures/S_SimplyChat` "" Message Type))))

(fn `Get SimplyChat`
  (returns (`SimplyChat Ref` :type "/Game/SimplyChat/Blueprint/ChatComponent/BP_SimplyChat Object Reference"))
  (return (`self.SimplyChat`)))

(fn `UserConstructionScript`)

(fn `UserName`
  (returns (UserName :type String))
  (bind _asbp_game_instance (cast `/Game/_DevelopersFolder/BP_GameInstance` (`GameplayStatics.GetGameInstance`)))
  (return (`/Game/_DevelopersFolder/BP_GameInstance.PlayerName` _asbp_game_instance)))