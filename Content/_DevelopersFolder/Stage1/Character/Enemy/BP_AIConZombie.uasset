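; AI controller for the zombie enemy that runs the BT_AIPatrol behavior tree on possess and tracks the player through AI perception.
; Sensing a LostChildPlayerBase actor cancels any pending timer and writes the target and line-of-sight flag to the Blackboard.
; Losing that actor starts a short grace timer that clears both keys on expiry, so the zombie keeps its target briefly after contact breaks.
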(event `self.ReceivePossess`
  (params (PossessedPawn :type "Pawn Object Reference"))
  (`self.RunBehaviorTree` "/Game/_DevelopersFolder/Stage1/Character/Enemy/BT_AIPatrol.BT_AIPatrol"))

(event `self.AIPerception.OnTargetPerceptionUpdated`
  (params (Actor :type "Actor Object Reference") (Stimulus :type "AIStimulus Structure"))
  (bind _blackboard (`self.Blackboard`))
  (bind _aslost_child_player_base (cast `/Game/_DevelopersFolder/Stage1/Character/Player/LostChildPlayerBase` Actor))
  (if (and (`KismetSystemLibrary.IsValid` _aslost_child_player_base) (`.bSuccessfullySensed` (break `AIStimulus` Stimulus)))
    (`KismetSystemLibrary.K2_ClearAndInvalidateTimerHandle` (`self.EventTimer`))
    (`BlackboardComponent.SetValueAsBool` _blackboard (`self.HasLineOfSight`) true)
    (`BlackboardComponent.SetValueAsObject` _blackboard (`self.EnemyActor`) Actor)
    (else
      (bind _returnvalue (`KismetSystemLibrary.K2_SetTimerDelegate` (delegate `StartEnemyTimer`) 4.0))
      (set `self.EventTimer` _returnvalue))))

(event `StartEnemyTimer`
  (bind _blackboard (`self.Blackboard`))
  (`BlackboardComponent.SetValueAsBool` _blackboard (`self.HasLineOfSight`) false)
  (`BlackboardComponent.SetValueAsObject` _blackboard (`self.EnemyActor`) null))

(fn `UserConstructionScript`)