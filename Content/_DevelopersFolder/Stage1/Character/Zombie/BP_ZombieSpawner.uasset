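; Zombie spawner actor that releases waves of BP_Zombie endlessly during play.
; BeginPlay starts a delayed timer for SpawnZombie, which spawns a batch and then re-arms its own timer at a shorter interval.
; Each zombie appears at a random reachable navmesh point within the Sphere component's radius, with random yaw, regardless of collision.
; ZombieCount increments once per batch rather than per zombie, and nothing here uses it to cap spawning.
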(event `self.ReceiveBeginPlay`
  (`KismetSystemLibrary.K2_SetTimer` null "SpawnZombie" 5.0))

(fn `SpawnZombie`
  (for _ (range 6)
    (`|SpawnActorFromClass` "/Game/_DevelopersFolder/Stage1/Character/Zombie/BP_Zombie.BP_Zombie_C" (`KismetMathLibrary.MakeTransform` (`NavigationSystemV1.K2_GetRandomReachablePointInRadius` (`self.K2_GetActorLocation`) (`SphereComponent.SphereRadius` (`self.Sphere`)) null null) (`KismetMathLibrary.MakeRotator` 0.0 0.0 (`KismetMathLibrary.RandomFloatInRange` 0.0 360.0))) "AlwaysSpawn" "OverrideRootScale" null null))
  (`/Engine/EditorBlueprintResources/StandardMacros.IncrementInt` (`self.ZombieCount`)
    (:`  `
      (`KismetSystemLibrary.K2_SetTimer` null "SpawnZombie" 3.0))))

(fn `UserConstructionScript`)