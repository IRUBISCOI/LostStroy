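; BP_Zombie is an AI zombie character that picks a random mesh at construction and spawns a name tag showing its HP.
; HP updates spawn blood effects, and attacks play a montage through a Req/Res event pair.
; Death uses the same pattern to count the kill in Stage1_GameState, stop AI logic and collision, then explode and destroy after a delay.
; StageClear deals damage equal to current HP without counting the kill.
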(event `self.ReceiveBeginPlay`
  (`self.SpawnNameTag`)
  (`self.SpawnDefaultController`))

(event `self.OnUpdateHp`
  (params (CurrentHp :type "Float (single-precision)") (MaxHp :type "Float (single-precision)"))
  (`parent.OnUpdateHp` CurrentHp MaxHp)
  (`NiagaraFunctionLibrary.SpawnSystemAtLocation` "/Game/BloodFX/FX/NS_BloodImpact_Big.NS_BloodImpact_Big" (`self.K2_GetActorLocation`) (`self.K2_GetActorRotation`))
  (`/Game/_DevelopersFolder/Stage1/Widget/NametagWidget.SetHp` (`self.NameTag`) CurrentHp MaxHp))

(event `Res_Ragdoll`
  (`KismetSystemLibrary.K2_SetTimer` null "ZombieDead" 3.0))

(event `self.DoRagdoll`
  (`self.Req_Ragdoll`))

(event `Req_Ragdoll`
  (`|ExecutionSequence`
    (:`then_0`
      (if (`self.IsUpdateKill`)
        (bind _asstage_1_game_state (cast `/Game/_DevelopersFolder/Stage1/Blueprints/Stage1_GameState` (`GameplayStatics.GetGameState`)))
        (set `/Game/_DevelopersFolder/Stage1/Blueprints/Stage1_GameState.TotalKill` (+ (`/Game/_DevelopersFolder/Stage1/Blueprints/Stage1_GameState.TotalKill` _asstage_1_game_state) 1) _asstage_1_game_state)))
    (:`then_1`
      (`BrainComponent.StopLogic` (`AIController.BrainComponent` (`AIBlueprintHelperLibrary.GetAIController` self)) "Dead"))
    (:`then_2`
      (`PrimitiveComponent.SetCollisionEnabled` (`self.Mesh`) "NoCollision"))
    (:`then_3`
      (`self.Res_Ragdoll`))))

(event `Req_Attack`
  (`self.Res_Attack`))

(event `Res_Attack`
  (`self.PlayAnimMontage` "/Game/_DevelopersFolder/Stage1/Character/Zombie/Animation/zombie_attack_Montage.zombie_attack_Montage" 1.5))

(event `/Game/_DevelopersFolder/Stage1/Blueprints/KillInterface.StageClear`
  (bind _bpc_zombiecomponent (`self.BPC_ZombieComponent`))
  (set `self.IsUpdateKill` false)
  (`ZombieComponent.AddDamage` _bpc_zombiecomponent (`ZombieComponent.GetCurHp` _bpc_zombiecomponent))
  (`KismetSystemLibrary.K2_SetTimer` null "ZombieDead" 3.0))

(event `self.ReceiveDestroyed`
  (`Widget.RemoveFromParent` (`self.NameTag`)))

(fn `SpawnNameTag`
  (bind _returnvalue (`|CreateWidget` "/Game/_DevelopersFolder/Stage1/Widget/NametagWidget.NametagWidget_C" null self))
  (bind _output_get (set `self.NameTag` _returnvalue))
  (`UserWidget.AddToViewport` _output_get 0))

(fn `UserConstructionScript`
  (`SkinnedMeshComponent.SetSkinnedAssetAndUpdate` (`self.Mesh`) (`KismetArrayLibrary.Array_Random` (`self.ListOfZombie`)) true))

(fn `ZombieAttack`
  (`self.Req_Attack`))

(fn `ZombieDead`
  (`NiagaraFunctionLibrary.SpawnSystemAtLocation` "/Game/BloodFX/FX/NS_BloodExplodeSmall.NS_BloodExplodeSmall" (`self.K2_GetActorLocation`) (`self.K2_GetActorRotation`))
  (`self.K2_DestroyActor`))