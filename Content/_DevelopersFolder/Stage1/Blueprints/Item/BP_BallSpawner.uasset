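; BP_BallSpawner is a timed spawner actor that emits random balls from BallList at its location with random yaw.
; On BeginPlay it starts a looping spawn timer, with a second timer ending spawning after a fixed period and a lifespan removing the spawner later.
; Two spheres act on exit: VisibleSphere reveals a ball's mesh and activates its particle, while DestroySphere destroys departing ItemObjects.
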(event `self.ReceiveBeginPlay`
  (`self.Req_SpawnBallStart`))

(event `Req_SpawnBallStart`
  (`self.SetLifeSpan` 40.0)
  (`KismetSystemLibrary.K2_SetTimer` null "SpawnBall" 0.2 true)
  (`KismetSystemLibrary.K2_SetTimerDelegate` (delegate `ClearTimer`) 20.0)
  (`KismetSystemLibrary.PrintString` "spawn timer"))

(event `ClearTimer`
  (`KismetSystemLibrary.K2_ClearTimer` null "SpawnBall"))

(event `self.DestroySphere.OnComponentEndOverlap`
  (params (OverlappedComponent :type "PrimitiveComponent Object Reference") (OtherActor :type "Actor Object Reference") (OtherComp :type "PrimitiveComponent Object Reference") (OtherBodyIndex :type Integer))
  (bind _asitem_object (cast `ItemObject` OtherActor))
  (`self.K2_DestroyActor` _asitem_object))

(event `self.VisibleSphere.OnComponentEndOverlap`
  (params (OverlappedComponent :type "PrimitiveComponent Object Reference") (OtherActor :type "Actor Object Reference") (OtherComp :type "PrimitiveComponent Object Reference") (OtherBodyIndex :type Integer))
  (bind _asbp_ball_base (cast `/Game/_DevelopersFolder/Stage1/Blueprints/Item/BP_BallBase` OtherActor))
  (`SceneComponent.SetVisibility` (`ItemObject.StaticMesh` _asbp_ball_base) true false)
  (`ActorComponent.SetActive` (`/Game/_DevelopersFolder/Stage1/Blueprints/Item/BP_BallBase.Particle` _asbp_ball_base) true false))

(fn `SpawnBall`
  (`|SpawnActorFromClass` (`KismetArrayLibrary.Array_Random` (`self.BallList`)) (`KismetMathLibrary.MakeTransform` (`self.K2_GetActorLocation`) (`KismetMathLibrary.MakeRotator` 0.0 0.0 (`KismetMathLibrary.RandomFloatInRange` 0.0 360.0))) "Undefined" "OverrideRootScale" null null))

(fn `UserConstructionScript`)