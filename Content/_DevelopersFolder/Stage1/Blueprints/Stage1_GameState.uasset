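; Stage 1 GameState that tracks the replicated kill count and ends the stage when it reaches the target.
; OnRep_TotalKill prints the count and sends kill updates to KillInterface actors and the local GameHUD.
; At CompleteKill, Stage1Complete broadcasts a clear message through the interface, calls CallClearStage on the first two LostChild players, then the SBJ level opens.
; An older direct clear of the zombie spawner and zombies remains unconnected.
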(fn `OnRep_TotalKill`
  (bind _totalkill (`self.TotalKill`))
  (`KismetSystemLibrary.PrintString` (`KismetStringLibrary.Concat_StrStr` "TotalKill : " (`KismetStringLibrary.Conv_IntToString` _totalkill)))
  (`|ExecutionSequence`
    (:`then_0`
      (bind _outactors (`GameplayStatics.GetAllActorsWithInterface` "/Game/_DevelopersFolder/Stage1/Blueprints/KillInterface.KillInterface_C"))
      (`|ExecutionSequence`
        (:`then_0`
          (message `/Game/_DevelopersFolder/Stage1/Blueprints/KillInterface.UpdateKill` _outactors))
        (:`then_1`
          (bind _asgame_hud (cast `GameHUD` (`PlayerController.GetHUD` (`GameplayStatics.GetPlayerController` 0))))
          (message `/Game/_DevelopersFolder/Stage1/Blueprints/KillInterface.UpdateKill` _asgame_hud))))
    (:`then_1`
      (if (>= _totalkill (`self.CompleteKill`))
        (`self.Stage 1 Complete`)
        (`GameplayStatics.OpenLevel` "SBJ")))))

(fn `Stage 1 Complete`
  (`|ExecutionSequence`
    (:`then_0`
      (bind _outactors (`GameplayStatics.GetAllActorsWithInterface` "/Game/_DevelopersFolder/Stage1/Blueprints/KillInterface.KillInterface_C"))
      (for _array_element _outactors
        (message `/Game/_DevelopersFolder/Stage1/Blueprints/KillInterface.StageClear` _array_element)))
    (:`then_1`
      (for _index (range 2)
        (bind _aslost_child (cast `/Game/_DevelopersFolder/Stage1/Character/Player/LostChild` (`GameplayStatics.GetPlayerCharacter` _index)))
        (`/Game/_DevelopersFolder/Stage1/Character/Player/LostChild.ClearStage` _aslost_child)))))

(fn `UserConstructionScript`)