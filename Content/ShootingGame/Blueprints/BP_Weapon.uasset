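; Hitscan weapon actor for the shooting game, configured by WeaponData and able to attach to a character or drop as a physics object.
; Input events play shoot and reload montages, while notify events handle effects, firing and magazine-based refills through ShootingPlayerState.
; Only the local player's character requests shots from the camera view, which consume ammo, then line-trace to damage characters.
; An Ammo OnRep updates the owning player's HUD.
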(event `self.ReceiveBeginPlay`
  (bind _weapondata_staticmesh (break `/Game/ShootingGame/Blueprints/ST_Weapon` (`self.WeaponData`)))
  (bind (_weapondata_staticmesh_2 _weapondata_shootmontage _weapondata_reloadmontage _weapondata_shootsound _weapondata_shooteffect _weapondata_maxammo) (break `/Game/ShootingGame/Blueprints/ST_Weapon` (`self.WeaponData`)))
  (`StaticMeshComponent.SetStaticMesh` (`self.StaticMesh`) _weapondata_staticmesh)
  (`AudioComponent.SetSound` (`self.Audio`) _weapondata_shootsound)
  (set `self.Ammo` _weapondata_maxammo))

(event `self.PressReload`
  (bind _owncharacter (`self.OwnCharacter`))
  (bind (_weapondata_staticmesh _weapondata_shootmontage _weapondata_reloadmontage) (break `/Game/ShootingGame/Blueprints/ST_Weapon` (`self.WeaponData`)))
  (bind _asshooting_player_state (cast `/Game/ShootingGame/GameMode/ShootingPlayerState` (`Pawn.PlayerState` _owncharacter)))
  (if (`/Game/ShootingGame/GameMode/ShootingPlayerState.IsCanUseMag` _asshooting_player_state)
    (`Character.PlayAnimMontage` _owncharacter _weapondata_reloadmontage 1.0 "None")))

(event `self.TriggerEvent`
  (params (IsPressed :type Boolean))
  (bind (_weapondata_staticmesh _weapondata_shootmontage) (break `/Game/ShootingGame/Blueprints/ST_Weapon` (`self.WeaponData`)))
  (if IsPressed
    (`Character.PlayAnimMontage` (`self.OwnCharacter`) _weapondata_shootmontage 1.0 "None")))

(event `self.NotifyShoot`
  (bind _returnvalue (`GameplayStatics.GetPlayerCameraManager` 0))
  (bind _iscanuse (`self.IsCanUse`))
  (if _iscanuse
    (`self.ShowShootEffect`)
    ;[1 1 1] 데미지 요청 처리
    (if (== (`self.OwnCharacter`) (`GameplayStatics.GetPlayerCharacter` 0))
      (`self.ReqShoot` (`self.K2_GetActorLocation` _returnvalue) (`self.GetActorForwardVector` _returnvalue)))))

(event `ReqShoot`
  (params (StartPoint :type "Vector Structure") (ForwardVector :type "Vector Structure"))
  (bind _iscanshoot (`self.UseAmmo`))
  (if _iscanshoot
    (`self.ProcessServerShoot` StartPoint ForwardVector)))

(event `self.NotifyReload`
  (`self.DoReload`))

(fn `AttachWeapon`
  (params (Character :type "Character Object Reference"))
  (returns (Result :type Boolean))
  (set `self.OwnCharacter` Character)
  (`PrimitiveComponent.SetSimulatePhysics` (`self.StaticMesh`) false)
  (`PrimitiveComponent.SetCollisionEnabled` (`self.StaticMesh`) "NoCollision")
  (`self.K2_AttachToComponent` (`Character.Mesh` Character) "weapon" "SnapToTarget" "SnapToTarget" "KeepWorld")
  (`self.UpdateAmmoToUI` (`self.Ammo`))
  (return false))

(fn `DetachWeapon`
  (returns (Result :type Boolean))
  (bind _staticmesh (`self.StaticMesh`))
  (`self.UpdateAmmoToUI` 0)
  (set `self.OwnCharacter` null)
  (`PrimitiveComponent.SetCollisionEnabled` _staticmesh "QueryAndPhysics")
  (`PrimitiveComponent.SetSimulatePhysics` _staticmesh true)
  (`SceneComponent.K2_DetachFromComponent` (`self.StaticMesh`) "KeepWorld" "KeepWorld" "KeepWorld" true)
  (return false))

(fn `DoReload`
  (bind (_weapondata_staticmesh _weapondata_shootmontage _weapondata_reloadmontage _weapondata_shootsound _weapondata_shooteffect _weapondata_maxammo) (break `/Game/ShootingGame/Blueprints/ST_Weapon` (`self.WeaponData`)))
  (bind _owncharacter (`self.OwnCharacter`))
  (`/Engine/EditorBlueprintResources/StandardMacros.IsValid` _owncharacter
    (:`Is Valid`
      (bind _asshooting_player_state (cast `/Game/ShootingGame/GameMode/ShootingPlayerState` (`Pawn.PlayerState` _owncharacter)))
      (bind _iscanuse (`/Game/ShootingGame/GameMode/ShootingPlayerState.UseMag` _asshooting_player_state))
      (if _iscanuse
        (set `self.Ammo` _weapondata_maxammo)))))

(fn `IsCanUse`
  (returns (IsCanUse :type Boolean))
  (bind _asshooting_character (cast `` (`self.OwnCharacter`))
    (:`then`
      (if (`/Game/ShootingGame/Blueprints/BP_Weapon.IsRagdoll` _asshooting_character)
        (return false)
        (else
          (return (> (`self.Ammo`) 0)))))
    (:`CastFailed`
      (return false))))

(fn `OnRep_Ammo`
  (bind _owncharacter (`self.OwnCharacter`))
  (`/Engine/EditorBlueprintResources/StandardMacros.IsValid` _owncharacter
    (:`Is Valid`
      (if (== (`Pawn.GetController` _owncharacter) (`GameplayStatics.GetPlayerController` 0))
        (`self.UpdateAmmoToUI` (`self.Ammo`))))))

(fn `ProcessServerShoot`
  (params (StartPoint :type "Vector Structure") (ForwardVector :type "Vector Structure"))
  (bind (_weapondata_staticmesh _weapondata_shootmontage _weapondata_reloadmontage _weapondata_shootsound _weapondata_shooteffect _weapondata_maxammo _weapondata_damage) (break `/Game/ShootingGame/Blueprints/ST_Weapon` (`self.WeaponData`)))
  (bind _outhit (`KismetSystemLibrary.LineTraceSingleForObjects` (+ StartPoint (* ForwardVector 350.0)) (+ StartPoint (* ForwardVector (`self.Distance`))) (`|MakeArray` "ObjectTypeQuery3" "ObjectTypeQuery1" "ObjectTypeQuery2" "ObjectTypeQuery4" "ObjectTypeQuery5" "ObjectTypeQuery6" :!type "EObjectTypeQuery Enum") false (`|MakeArray` (`self.OwnCharacter`) :!type "Actor Object Reference") "Persistent"))
  (bind _ascharacter (cast `Character` (`.HitActor` (`GameplayStatics.BreakHitResult` _outhit))))
  (`GameplayStatics.ApplyDamage` _ascharacter _weapondata_damage (`Pawn.GetController` (`self.OwnCharacter`)) self))

(fn `ShowShootEffect`
  (bind (_weapondata_staticmesh _weapondata_shootmontage _weapondata_reloadmontage _weapondata_shootsound _weapondata_shooteffect) (break `/Game/ShootingGame/Blueprints/ST_Weapon` (`self.WeaponData`)))
  (bind (_returnvalue_location _returnvalue_rotation) (`KismetMathLibrary.BreakTransform` (`SceneComponent.GetSocketTransform` (`self.StaticMesh`) "Muzzle" "RTS_World")))
  (`GameplayStatics.SpawnEmitterAtLocation` _weapondata_shooteffect _returnvalue_location _returnvalue_rotation (0.3 0.3 0.3) true "AutoRelease")
  (`AudioComponent.Play` (`self.Audio`) 0.0))

(fn `UpdateAmmoToUI`
  (params (Ammo :type Integer))
  (bind _returnvalue (`GameplayStatics.GetPlayerController` 0))
  (bind _owncharacter (`self.OwnCharacter`))
  (`/Engine/EditorBlueprintResources/StandardMacros.IsValid` _owncharacter
    (:`Is Valid`
      (if (== (`Pawn.GetController` _owncharacter) _returnvalue)
        (bind _asshooting_hud (cast `/Game/ShootingGame/GameMode/ShootingHud` (`PlayerController.GetHUD` _returnvalue)))
        (`/Game/ShootingGame/Widget/HudWidget.SetAmmo` (`/Game/ShootingGame/GameMode/ShootingHud.HudWidget` _asshooting_hud) Ammo)))))

(fn `UseAmmo`
  (returns (IsCanShoot :type Boolean))
  (locals (CanUsed :type Boolean))
  (set `local.CanUsed` (> (`self.Ammo`) 0))
  (set `self.Ammo` (`KismetMathLibrary.Clamp` (- (`self.Ammo`) 1) 0 30))
  (return (`local.CanUsed`)))

(fn `UserConstructionScript`)